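; Base tower Blueprint for a tower defense game, providing targeting, turret aiming and shared tower hooks.
; Each tick it picks a target from EnemiesInRange by focus mode (path order, health or speed) and smoothly yaws the top toward it unless overheated.
; Events handle support-tower buffs, upgrade sell value, damage text and range display; destruction notifies the supporting tower.
; Firing is absent here, and stat getters return placeholder defaults.
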(event Custom|OnDestroyed_Event
  (params (DestroyedActor :type Actor%20Object%20Reference))
  (bind _supvfx (Variables|Default|GetSupVfx))
  (bind _suptower (Variables|Default|GetSupTower))
  ;[0.15 0.15 0.15 0.5] Beginplay
  (Utilities|IsValid _suptower
    (:Is%20Valid
      (CallFunction|TowerSold _suptower self))
    (:Is%20Not%20Valid
      _))
  (Utilities|IsValid _supvfx
    (:Is%20Valid
      (Components|Activation|Deactivate _supvfx))))

(event Custom|SelectTarget
  ;[0.15 0.15 0.15 0.5] SelectTarget
  (switch string (Variables|Default|GetFocus%20Type)
    (:First
      (Variables|Default|SetMaxDistance 0.0)
      (if (> (Utilities|Array|Length (Variables|Default|GetEnemiesInRange)) 0)
        (for _array_element (Variables|Default|GetEnemiesInRange)
          (bind _length (Class|BPIEnemy|GetLength(Message) _array_element))
          (if (> _length (Variables|Default|GetMaxDistance))
            (Variables|Default|SetMaxDistance _length)
            (Variables|Default|SetCurrentTarget _array_element)
            (bind _currenthealth (Class|BPIEnemy|GetEnemyHealth(Message) _array_element))
            (if (<= _currenthealth 0.0)
              (Utilities|Array|RemoveItem (Variables|Default|GetEnemiesInRange) _array_element))))
        (else
          (Variables|Default|SetCurrentTarget 0))))
    (:Last
      (Variables|Default|SetMaxDistance 1e+19)
      (if (> (Utilities|Array|Length (Variables|Default|GetEnemiesInRange)) 0)
        (for _array_element_2 (Variables|Default|GetEnemiesInRange)
          (bind _length_2 (Class|BPIEnemy|GetLength(Message) _array_element_2))
          (if (< _length_2 (Variables|Default|GetMaxDistance))
            (Variables|Default|SetMaxDistance _length_2)
            (Variables|Default|SetCurrentTarget _array_element_2)
            (bind _currenthealth_2 (Class|BPIEnemy|GetEnemyHealth(Message) _array_element_2))
            (if (<= _currenthealth_2 0.0)
              (Utilities|Array|RemoveItem (Variables|Default|GetEnemiesInRange) _array_element_2))))
        (else
          (Variables|Default|SetCurrentTarget 0))))
    (:Least%20Health
      (Variables|Default|SetEnemyHealth 1e+10)
      (if (> (Utilities|Array|Length (Variables|Default|GetEnemiesInRange)) 0)
        (for _array_element_3 (Variables|Default|GetEnemiesInRange)
          (bind _currenthealth_3 (Class|BPIEnemy|GetEnemyHealth(Message) _array_element_3))
          (if (< _currenthealth_3 (Variables|Default|GetEnemyHealth))
            (Variables|Default|SetEnemyHealth _currenthealth_3)
            (Variables|Default|SetCurrentTarget _array_element_3)
            (bind _currenthealth_4 (Class|BPIEnemy|GetEnemyHealth(Message) _array_element_3))
            (if (<= _currenthealth_4 0.0)
              (Utilities|Array|RemoveItem (Variables|Default|GetEnemiesInRange) _array_element_3))))
        (else
          (Variables|Default|SetCurrentTarget 0))))
    (:Most%20Health
      (Variables|Default|SetEnemyHealth 0.0)
      (if (> (Utilities|Array|Length (Variables|Default|GetEnemiesInRange)) 0)
        (for _array_element_4 (Variables|Default|GetEnemiesInRange)
          (bind _currenthealth_5 (Class|BPIEnemy|GetEnemyHealth(Message) _array_element_4))
          (if (> _currenthealth_5 (Variables|Default|GetEnemyHealth))
            (Variables|Default|SetEnemyHealth _currenthealth_5)
            (Variables|Default|SetCurrentTarget _array_element_4)
            (bind _currenthealth_6 (Class|BPIEnemy|GetEnemyHealth(Message) _array_element_4))
            (if (<= _currenthealth_6 0.0)
              (Utilities|Array|RemoveItem (Variables|Default|GetEnemiesInRange) _array_element_4))))
        (else
          (Variables|Default|SetCurrentTarget 0))))
    (:Slowest
      (Variables|Default|SetEnemySpeed 1e+14)
      (if (> (Utilities|Array|Length (Variables|Default|GetEnemiesInRange)) 0)
        (for _array_element_5 (Variables|Default|GetEnemiesInRange)
          (bind _enemyspeed (Class|BPIEnemy|GetEnemySpeed(Message) _array_element_5))
          (if (< _enemyspeed (Variables|Default|GetEnemySpeed))
            (Variables|Default|SetEnemySpeed _enemyspeed)
            (Variables|Default|SetCurrentTarget _array_element_5)
            (bind _currenthealth_7 (Class|BPIEnemy|GetEnemyHealth(Message) _array_element_5))
            (if (<= _currenthealth_7 0.0)
              (Utilities|Array|RemoveItem (Variables|Default|GetEnemiesInRange) _array_element_5))))
        (else
          (Variables|Default|SetCurrentTarget 0))))
    (:Fastest
      (Variables|Default|SetEnemySpeed 0.0)
      (if (> (Utilities|Array|Length (Variables|Default|GetEnemiesInRange)) 0)
        (for _array_element_6 (Variables|Default|GetEnemiesInRange)
          (bind _enemyspeed_2 (Class|BPIEnemy|GetEnemySpeed(Message) _array_element_6))
          (if (> _enemyspeed_2 (Variables|Default|GetEnemySpeed))
            (Variables|Default|SetEnemySpeed _enemyspeed_2)
            (Variables|Default|SetCurrentTarget _array_element_6)
            (bind _currenthealth_8 (Class|BPIEnemy|GetEnemyHealth(Message) _array_element_6))
            (if (<= _currenthealth_8 0.0)
              (Utilities|Array|RemoveItem (Variables|Default|GetEnemiesInRange) _array_element_6))))
        (else
          (Variables|Default|SetCurrentTarget 0))))))

(event EventBeginPlay
  (bind _towerrange (Variables|Default|GetTowerRange))
  (bind _boxextent (Collision|GetComponentBounds _towerrange))
  ;[0.15 0.15 0.15 0.5] Beginplay
  (Components|Box|SetBoxExtent (Variables|Default|GetBox) (Math|Vector|MakeVector (.x _boxextent) (.y _boxextent) 4.5e+02) true)
  (EventDispatchers|BindEventtoOnDestroyed (delegate Custom|OnDestroyed_Event)))

(event EventShowHideRange
  (params (bIsOpen :type Boolean))
  (bind _towerrange (Variables|Default|GetTowerRange))
  ;[0.15 0.15 0.15 0.5] Range
  (if bIsOpen
    (Rendering|SetVisibility _towerrange true false)
    (else
      (Rendering|SetVisibility _towerrange false false))))

(event EventChangeFocus
  (params (FocusType :type String))
  ;[0.15 0.15 0.15 0.5] Interface
  (Variables|Default|SetFocus%20Type FocusType))

(event EventUpdateInstalled
  (params (UpdatePrice :type Integer) (UpdateNumber :type Integer) (bGecici :type Boolean))
  (bind _returnvalue (Transformation|GetActorLocation))
  ;[0.15 0.15 0.15 0.5] Interface
  (Variables|Default|SetTowerSellPrice (+ (/ (* UpdatePrice 35) 100) (Variables|Default|GetTowerSellPrice)))
  (Niagara|SpawnSystematLocation "/Game/_Game/Niagara/NS_TowerLevelUp.NS_TowerLevelUp" (Math|Vector|MakeVector (.x _returnvalue) (.y _returnvalue) (+ (.z _returnvalue) 65.0))))

(event EventTick
  (params (DeltaSeconds :type Float%20%28single-precision%29))
  (bind _currenttarget (Variables|Default|GetCurrentTarget))
  (bind _towertop (Variables|Default|GetTowerTop))
  (bind _towertop_2 (Variables|Default|GetTowerTop))
  (bind _returnvalue (Transformation|GetWorldLocation _towertop))
  (bind _returnvalue_2 (Transformation|GetActorLocation _currenttarget))
  (bind _returnvalue_3 (Transformation|GetWorldRotation _towertop_2))
  (bind _returnvalue_4 (Math|Rotator|FindLookatRotation _returnvalue _returnvalue_2))
  ;[0.15 0.15 0.15 0.5] Tick
  (CallFunction|SelectTarget)
  (Variables|Default|GetCurrentTarget
    (:then
      (if (not (Variables|Default|GetbIsOverheated))
        (Transformation|SetWorldRotation _towertop_2 (Math|Rotator|MakeRotator (.roll _returnvalue_3) (.pitch _returnvalue_3) (.yaw (Math|Interpolation|RInterpTo (Transformation|GetWorldRotation _towertop) (Math|Rotator|MakeRotator (.roll _returnvalue_4) (.pitch _returnvalue_4) (+ (.yaw _returnvalue_4) 9e+01)) (Utilities|Time|GetWorldDeltaSeconds) 1e+01))) false false)))
    (:else)))

(event EventThermalControlSkillUse
  ;[0.15 0.15 0.15 0.5] Tick
  (Variables|Default|SetbCanOverheat false)
  (Development|PrintString "Hello"))

(event EventBulletHit
  (params (HittedEnemy :type Actor%20Object%20Reference) (Damage :type Float%20%28double-precision%29) (bIsCrit :type Boolean))
  ;[0.15 0.15 0.15 0.5] Interface
  (Utilities|IsValid HittedEnemy
    (:Is%20Valid
      (Game|SpawnActorfromClass "/Game/_Game/BP/BP_DamageText.BP_DamageText_C" (Math|Transform|MakeTransform (+ (Transformation|GetActorLocation HittedEnemy) "0.000000,0.000000,120.000000") "0, 0, 0" "1.000000,1.000000,1.000000") "Undefined" "MultiplyWithRoot" 0 Damage bIsCrit "" 0))))

(event EventSupportTower
  (params (SupportDamage :type Float%20%28double-precision%29) (SupportAttackSpeed :type Float%20%28double-precision%29) (SupportCritChance :type Float%20%28double-precision%29) (SupportCritMult :type Float%20%28double-precision%29) (Tower :type BP%20Tower%20Support%20Object%20Reference))
  ;[0.15 0.15 0.15 0.5] Interface
  (Variables|SupBuff|SetSupport%20Damage (* SupportDamage 1e+02))
  (Variables|SupBuff|SetSupport%20Attack%20Speed (* SupportAttackSpeed 1e+02))
  (Variables|SupBuff|SetSupport%20Crit%20Chance (* SupportCritChance 1e+02))
  (Variables|SupBuff|SetSupport%20Crit%20Mult SupportCritMult)
  (Variables|Default|SetSupTower Tower)
  (Variables|Default|SetbIsGetSupport true)
  (bind _supvfx (Variables|Default|GetSupVfx)
    (:then
      _)
    (:else
      (bind _returnvalue (Niagara|SpawnSystematLocation "/Game/_Game/Niagara/NS_SupBuff.NS_SupBuff" (Transformation|GetActorLocation)))
      (bind _output_get (Variables|Default|SetSupVfx _returnvalue))))
  (Components|Activation|Activate _output_get false))

(event EventRemoveSupport
  (bind _supvfx (Variables|Default|GetSupVfx))
  ;[0.15 0.15 0.15 0.5] Interface
  (Variables|Default|SetSupTower 0)
  (Variables|Default|SetbIsGetSupport false)
  (Utilities|IsValid _supvfx
    (:Is%20Valid
      (Components|Activation|Deactivate _supvfx))
    (:Is%20Not%20Valid
      _))
  (Variables|SupBuff|SetSupport%20Damage 0.0)
  (Variables|SupBuff|SetSupport%20Attack%20Speed 0.0)
  (Variables|SupBuff|SetSupport%20Crit%20Chance 0.0)
  (Variables|SupBuff|SetSupport%20Crit%20Mult 1.0))

(fn ConstructionScript)

(fn OverheatAnimActivete
  (Components|Activation|Activate (Variables|Default|GetSmoke) false))

(fn OverheatAnimDeActivete
  (Components|Activation|Deactivate (Variables|Default|GetSmoke)))

(fn GetIsGhostTower
  (return false))

(fn GetIsTowerGetSupport
  (return (Variables|Default|GetbIsGetSupport)))

(fn GetTile
  (return (Variables|Default|GetTile)))

(fn GetTowerGrid
  (return (Variables|Default|GetTile)))

(fn GetTowerStats
  (return 0.0 0.0 0.0 0.0 0.0 0.0 0.0 0.0 0.0 0.0 0.0))

(fn IsTowerSupport
  (return false))