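; Surge tower for a tower defense game that damages enemies with expanding Tesla waves, using stats from BP_Instance.
; Enemies entering its range box start a looping timer that adds heat and, given a valid target, spawns a Niagara wave.
; A timeline grows a collision sphere alongside the wave, damaging each enemy it overlaps.
; Overheating tilts the top and pauses attacks until cooldown; damage, waves, overheats, kills and credits are tracked.
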(event OnComponentBeginOverlap(Box)
  (params (OverlappedComponent :type Primitive%20Component%20Object%20Reference) (OtherActor :type Actor%20Object%20Reference) (OtherComp :type Primitive%20Component%20Object%20Reference) (OtherBodyIndex :type Integer) (bFromSweep :type Boolean) (SweepResult :type Hit%20Result%20Structure%20%28by%20ref%29))
  ;[0.15 0.15 0.15 0.5] Overlap
  (if (Utilities|DoesObjectImplementInterface OtherActor "/Game/_Game/BP/Frameworks/BPI_Enemy.BPI_Enemy_C")
    (Utilities|Array|Add (Variables|Default|GetEnemiesInRange) OtherActor)
    (if (Variables|Default|GetbIsTargetingEnemy)
      _
      (else
        (Variables|Default|SetbIsTargetingEnemy true)))
    (if (not (Utilities|Time|IsTimerActivebyHandle (Variables|Default|GetAttackTimerHandle)))
      (bind _returnvalue (Utilities|Time|SetTimerbyEvent (delegate Custom|AttackEnemyEvent) (.TowerSpeed (Utilities|Struct|BreakStructure_SurgeTower (Variables|/Game/_Game/BP/Frameworks/BP_Instance.BP_Instance_C|GetSurgeStats (Variables|Default|GetAs%20BP%20Instance)))) true))
      (Variables|Default|SetAttackTimerHandle _returnvalue))))

(event OnComponentEndOverlap(Box)
  (params (OverlappedComponent :type Primitive%20Component%20Object%20Reference) (OtherActor :type Actor%20Object%20Reference) (OtherComp :type Primitive%20Component%20Object%20Reference) (OtherBodyIndex :type Integer))
  (bind _enemiesinrange (Variables|Default|GetEnemiesInRange))
  ;[0.15 0.15 0.15 0.5] Overlap
  (if (Utilities|DoesObjectImplementInterface OtherActor "/Game/_Game/BP/Frameworks/BPI_Enemy.BPI_Enemy_C")
    (Utilities|Array|RemoveItem _enemiesinrange OtherActor)
    (if (== OtherActor (Variables|Default|GetCurrentTarget))
      (CallFunction|SelectTarget)
      (if (Utilities|Array|IsEmpty _enemiesinrange)
        (Variables|Default|SetbIsTargetingEnemy false)))))

(event OnComponentBeginOverlap(WaveCollision)
  (params (OverlappedComponent :type Primitive%20Component%20Object%20Reference) (OtherActor :type Actor%20Object%20Reference) (OtherComp :type Primitive%20Component%20Object%20Reference) (OtherBodyIndex :type Integer) (bFromSweep :type Boolean) (SweepResult :type Hit%20Result%20Structure%20%28by%20ref%29))
  (bind _enemiesinrange (Variables|Default|GetEnemiesInRange))
  (bind _as_bp_instance (Variables|Default|GetAs%20BP%20Instance))
  (bind _surgestats (Variables|/Game/_Game/BP/Frameworks/BP_Instance.BP_Instance_C|GetSurgeStats _as_bp_instance))
  (bind (_basetowerstats _towerdamage _towerspeed) (Utilities|Struct|BreakStructure_SurgeTower _surgestats))
  ;[0.15 0.15 0.15 0.5] Overlap
  (if (Utilities|DoesObjectImplementInterface OtherActor "/Game/_Game/BP/Frameworks/BPI_Enemy.BPI_Enemy_C")
    (Utilities|IsValid OtherActor
      (:Is%20Valid
        (Game|SpawnActorfromClass "/Game/_Game/BP/BP_DamageText.BP_DamageText_C" (Math|Transform|MakeTransform (+ (Transformation|GetActorLocation OtherActor) "0.000000,0.000000,120.000000") "0, 0, 0" "1.000000,1.000000,1.000000") "Undefined" "MultiplyWithRoot" 0 _towerdamage false 0)
        (Variables|InGameStats|SetTotalDamageDealt (+ _towerdamage (Variables|InGameStats|GetTotalDamageDealt)))
        (bind (_currenthealth _maxhealth) (Class|BPIEnemy|GetEnemyHealth(Message) OtherActor))
        (Class|BPIEnemy|SetHealth(Message) OtherActor (- _currenthealth _towerdamage) _maxhealth)
        (bind _currenthealth_2 (Class|BPIEnemy|GetEnemyHealth(Message) OtherActor))
        (if (<= _currenthealth_2 0.0)
          (Utilities|Array|RemoveItem _enemiesinrange OtherActor)
          (Math|Float|IncrementFloat (Variables|InGameStats|GetAVG)
            (:%20%20
              (if (Utilities|Array|IsEmpty _enemiesinrange)
                (Variables|Default|SetbIsTargetingEnemy false))
              (Class|BPIEnemy|EnemyKilled(Message) OtherActor self))))))))

(event Custom|AttackEnemyEvent
  (bind _as_bp_instance (Variables|Default|GetAs%20BP%20Instance))
  (bind _as_bp_instance_2 (Variables|Default|GetAs%20BP%20Instance))
  (bind _towertop (Variables|Default|GetTowerTop))
  (bind _enemiesinrange (Variables|Default|GetEnemiesInRange))
  (bind _wavecollision (Variables|Default|GetWaveCollision))
  (bind _damagetimeline (Variables|Default|GetDamageTimeline))
  (bind _surgestats (Variables|/Game/_Game/BP/Frameworks/BP_Instance.BP_Instance_C|GetSurgeStats _as_bp_instance))
  (bind _surgestats_2 (Variables|/Game/_Game/BP/Frameworks/BP_Instance.BP_Instance_C|GetSurgeStats _as_bp_instance_2))
  (bind _relativerotation (Variables|/Script/Engine.SceneComponent|GetRelativeRotation _towertop))
  (bind _towerspeed (Utilities|Struct|BreakStructure_SurgeTower _surgestats_2))
  (bind (_basetowerstats _towerdamage _towerspeed_2) (Utilities|Struct|BreakStructure_SurgeTower _surgestats))
  (bind (_towerrange _toweroverheattime _toweroverheatduration) (Utilities|Struct|BreakStructure_TowerBase _basetowerstats))
  ;[0.15 0.15 0.15 0.5] Overlap
  (Utilities|FlowControl|Sequence
    (:then_0
      (if (and (or (Variables|Default|GetbIsOverheated) (not (Variables|Default|GetbIsTargetingEnemy))) (and (> (Variables|Default|GetCurrentHeat) 0.0) (< (Variables|Default|GetCurrentHeat) _toweroverheattime)))
        (Variables|Default|SetCurrentHeat (- (Variables|Default|GetCurrentHeat) _towerspeed_2))))
    (:then_1
      (if (and (Variables|Default|GetbIsTargetingEnemy) (not (Variables|Default|GetbIsOverheated)))
        (Utilities|FlowControl|Sequence
          (:then_0
            (if (Variables|Default|GetbIsTargetingEnemy)
              (bind _output_get (Variables|Default|SetCurrentHeat (+ _towerspeed_2 (Variables|Default|GetCurrentHeat))))
              (if (>= _output_get _toweroverheattime)
                (Math|Float|IncrementFloat (Variables|InGameStats|GetOverheatCount)
                  (:%20%20
                    (Variables|Default|SetbIsOverheated true)
                    (Utilities|FlowControl|Sequence
                      (:then_0
                        (bind _a (Timeline|Timeline_0 PlayFromStart)
                          (:Update
                            (Transformation|SetRelativeRotation _towertop (Math|Rotator|MakeRotator (Math|Float|Lerp 0.0 -2e+01 _a) (.pitch _relativerotation) (.yaw _relativerotation)) false false))
                          (:Finished
                            (Utilities|FlowControl|DoOnce false) ; enters at Reset
                          )))
                      (:then_1
                        (Utilities|FlowControl|DoOnce false
                          (:Completed
                            (CallFunction|OverheatAnimActivete)
                            (Utilities|Time|SetTimerbyEvent (delegate Custom|OverHeatCoolDown) _toweroverheatduration))))))))))
          (:then_1
            (Utilities|IsValid (Variables|Default|GetCurrentTarget)
              (:Is%20Valid
                (Math|Float|IncrementFloat (Variables|InGameStats|GetTotalWawesEmitted)
                  (:%20%20
                    (bind _returnvalue (Niagara|SpawnSystematLocation "/Game/_Game/Niagara/NS_TeslaWave.NS_TeslaWave" (.location (Transformation|GetWorldTransform (Variables|Default|GetBulletSpawnPoint)))))
                    (Niagara|SetNiagaraVariable(Float) _returnvalue "User.WaveSize" (* (.y (.BoxExtent (Collision|GetComponentBounds (Variables|Default|GetTowerRange)))) 3.0))
                    (Niagara|SetNiagaraVariable(Float) _returnvalue "User.TowerSpeed" _towerspeed)
                    (Components|Timeline|SetTimelineLength _damagetimeline _towerspeed)
                    (Components|Timeline|SetPlayRate _damagetimeline (/ 1.0 _towerspeed))
                    (bind _a_2 (Timeline|DamageTimeline PlayFromStart)
                      (:Update
                        (Components|Sphere|SetSphereRadius _wavecollision (Math|Float|Lerp 0.0 (.x (.BoxExtent (Collision|GetComponentBounds (Variables|Default|GetTowerRange)))) _a_2) true))
                      (:Finished
                        (Components|Sphere|SetSphereRadius _wavecollision 0.0 true)))))))))))))

(event Custom|OverHeatCoolDown
  (bind _towertop (Variables|Default|GetTowerTop))
  (bind _enemiesinrange (Variables|Default|GetEnemiesInRange))
  (bind _relativerotation (Variables|/Script/Engine.SceneComponent|GetRelativeRotation _towertop))
  ;[0.15 0.15 0.15 0.5] Overlap
  (Variables|Default|SetCurrentHeat 0.0)
  (Variables|Default|SetbIsOverheated false)
  (Utilities|FlowControl|Sequence
    (:then_0
      (bind _a (Timeline|Timeline Play)
        (:Update
          (Transformation|SetRelativeRotation _towertop (Math|Rotator|MakeRotator (Math|Float|Lerp -2e+01 0.0 _a) (.pitch _relativerotation) (.yaw _relativerotation)) false false))))
    (:then_1
      (Utilities|FlowControl|DoOnce false
        (:Completed
          (CallFunction|OverheatAnimDeActivete)
          (for _array_element _enemiesinrange
            (Utilities|IsValid _array_element
              (:Is%20Not%20Valid
                (Utilities|Array|RemoveItem _enemiesinrange _array_element))))
          (if (Utilities|Array|IsEmpty _enemiesinrange)
            (Variables|Default|SetbIsTargetingEnemy false)))))
    (:then_2
      (Utilities|FlowControl|DoOnce false) ; enters at Reset
    )))

(event EventBeginPlay
  (bind _towerrange (Variables|Default|GetTowerRange))
  ;[0.15 0.15 0.15 0.5] Beginplay
  (bind _asbp_instance (Utilities|Casting|CastToBP_Instance (Game|GetGameInstance)))
  (Variables|Default|SetAs%20BP%20Instance _asbp_instance)
  (Variables|Default|SetTower self)
  (Rendering|SetVisibility _towerrange false false)
  (Transformation|SetRelativeScale3D (Variables|Default|GetTowerRange) (* (Variables|/Script/Engine.SceneComponent|GetRelativeScale3D (Variables|Default|GetExample)) 8.0))
  (Transformation|SetRelativeScale3D _towerrange (* (Variables|/Script/Engine.SceneComponent|GetRelativeScale3D _towerrange) (.TowerRange (Utilities|Struct|BreakStructure_TowerBase (.BaseTowerStats (Utilities|Struct|BreakStructure_SurgeTower (Variables|/Game/_Game/BP/Frameworks/BP_Instance.BP_Instance_C|GetSurgeStats (Variables|Default|GetAs%20BP%20Instance)))))) 0.9))
  (|CallParentFunction))

(event EventTick
  (params (DeltaSeconds :type Float%20%28single-precision%29))
  ;[0.15 0.15 0.15 0.5] Tick
  (|CallParentFunction DeltaSeconds))

(event EventEnemyDied
  (params (DropMoney :type Float%20%28double-precision%29))
  (bind _returnvalue (Game|Player|GetPlayerPawn 0))
  ;[0.15 0.15 0.15 0.5] Interface
  (Variables|InGameStats|SetTotalCreditEarned (+ DropMoney (Variables|InGameStats|GetTotalCreditEarned)))
  (bind _money (Class|BPIGeneral|GetMoney(Message) _returnvalue))
  (Class|BPIGeneral|MoneyChanged(Message) _returnvalue (Math|Float|Truncate (+ _money DropMoney))))

(fn ConstructionScript
  (|CallParentFunction))

(fn GetTowerStats
  (return (Variables|InGameStats|GetTotalDamageDealt) 0.0 0.0 (Variables|InGameStats|GetOverheatCount) (Variables|InGameStats|GetTotalCreditEarned) (Variables|Default|GetTowerSellPrice) (Variables|Default|GetCurrentHeat) 0.0 (Variables|InGameStats|GetTotalWawesEmitted) (Variables|InGameStats|GetAVG) 0.0))