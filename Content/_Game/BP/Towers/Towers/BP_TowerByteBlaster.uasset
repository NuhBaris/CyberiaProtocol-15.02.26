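; Byte Blaster tower that shoots bullets at enemies in range, using ByteStats from the game instance.
; Range-box overlaps track enemies and start a looping attack timer that spawns bullets and builds heat, or cools when idle.
; Overheating halts fire and tilts the turret top until a timed cooldown.
; Bullet hits roll crits, damage the current target through interface messages, report kills, and record tower stats; kill rewards credit the player.
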(event OnComponentBeginOverlap(Box)
  (params (OverlappedComponent :type Primitive%20Component%20Object%20Reference) (OtherActor :type Actor%20Object%20Reference) (OtherComp :type Primitive%20Component%20Object%20Reference) (OtherBodyIndex :type Integer) (bFromSweep :type Boolean) (SweepResult :type Hit%20Result%20Structure%20%28by%20ref%29))
  ;[0.15 0.15 0.15 0.5] Overlap
  (if (Utilities|DoesObjectImplementInterface OtherActor "/Game/_Game/BP/Frameworks/BPI_Enemy.BPI_Enemy_C")
    (Utilities|Array|Add (Variables|Default|GetEnemiesInRange) OtherActor)
    (if (Variables|Default|GetbIsTargetingEnemy)
      _
      (else
        (Variables|Default|SetbIsTargetingEnemy true)))
    (if (not (Utilities|Time|IsTimerActivebyHandle (Variables|Default|GetAttackTimerHandle)))
      (bind _returnvalue (Utilities|Time|SetTimerbyEvent (delegate Custom|AttackEnemyEvent) (.TowerSpeed (Utilities|Struct|BreakStructure_ByteBlaster (Variables|/Game/_Game/BP/Frameworks/BP_Instance.BP_Instance_C|GetByteStats (Variables|Default|GetAs%20BP%20Instance)))) true))
      (Variables|Default|SetAttackTimerHandle _returnvalue))))

(event OnComponentEndOverlap(Box)
  (params (OverlappedComponent :type Primitive%20Component%20Object%20Reference) (OtherActor :type Actor%20Object%20Reference) (OtherComp :type Primitive%20Component%20Object%20Reference) (OtherBodyIndex :type Integer))
  (bind _enemiesinrange (Variables|Default|GetEnemiesInRange))
  ;[0.15 0.15 0.15 0.5] Overlap
  (if (Utilities|DoesObjectImplementInterface OtherActor "/Game/_Game/BP/Frameworks/BPI_Enemy.BPI_Enemy_C")
    (Utilities|Array|RemoveItem _enemiesinrange OtherActor)
    (if (== OtherActor (Variables|Default|GetCurrentTarget))
      (CallFunction|SelectTarget)
      (if (Utilities|Array|IsEmpty _enemiesinrange)
        (Variables|Default|SetbIsTargetingEnemy false)))))

(event Custom|AttackEnemyEvent
  (bind _towertop (Variables|Default|GetTowerTop))
  (bind _enemiesinrange (Variables|Default|GetEnemiesInRange))
  (bind _as_bp_instance (Variables|Default|GetAs%20BP%20Instance))
  (bind _currenttarget (Variables|Default|GetCurrentTarget))
  (bind _bulletspawnpoint (Variables|Default|GetBulletSpawnPoint))
  (bind _relativerotation (Variables|/Script/Engine.SceneComponent|GetRelativeRotation _towertop))
  (bind _bytestats (Variables|/Game/_Game/BP/Frameworks/BP_Instance.BP_Instance_C|GetByteStats _as_bp_instance))
  (bind (_basetowerstats _towerdamage _towerspeed) (Utilities|Struct|BreakStructure_ByteBlaster _bytestats))
  (bind (_towerrange _toweroverheattime _toweroverheatduration) (Utilities|Struct|BreakStructure_TowerBase _basetowerstats))
  ;[0.15 0.15 0.15 0.5] Overlap
  (Utilities|FlowControl|Sequence
    (:then_0
      (if (and (or (Variables|Default|GetbIsOverheated) (not (Variables|Default|GetbIsTargetingEnemy))) (and (> (Variables|Default|GetCurrentHeat) 0.0) (< (Variables|Default|GetCurrentHeat) _toweroverheattime)))
        (Variables|Default|SetCurrentHeat (- (Variables|Default|GetCurrentHeat) _towerspeed))))
    (:then_1
      (if (and (Variables|Default|GetbIsTargetingEnemy) (not (Variables|Default|GetbIsOverheated)))
        (Utilities|FlowControl|Sequence
          (:then_0
            (if (Variables|Default|GetbIsTargetingEnemy)
              (bind _output_get (Variables|Default|SetCurrentHeat (+ _towerspeed (Variables|Default|GetCurrentHeat))))
              (if (>= _output_get _toweroverheattime)
                (Math|Float|IncrementFloat (Variables|InGameStats|GetOverheatCount)
                  (:%20%20
                    (Variables|Default|SetbIsOverheated true)
                    (Utilities|FlowControl|Sequence
                      (:then_0
                        (bind _a (Timeline|Timeline_0 PlayFromStart)
                          (:Update
                            (Transformation|SetRelativeRotation _towertop (Math|Rotator|MakeRotator (Math|Float|Lerp 0.0 -2e+01 _a) (.pitch _relativerotation) (.yaw _relativerotation)) false false))
                          (:Finished
                            (Utilities|FlowControl|DoOnce false) ; enters at Reset
                          )))
                      (:then_1
                        (Utilities|FlowControl|DoOnce false
                          (:Completed
                            (CallFunction|OverheatAnimActivete)
                            (Utilities|Time|SetTimerbyEvent (delegate Custom|OverHeatCoolDown) _toweroverheatduration))))))))))
          (:then_1
            (Utilities|IsValid _currenttarget
              (:Is%20Valid
                (Niagara|SpawnSystematLocation "/Game/_Game/Niagara/NS_Muzzle.NS_Muzzle" (.location (Transformation|GetWorldTransform _bulletspawnpoint)))
                (bind _returnvalue (Game|SpawnActorfromClass "/Game/_Game/BP/BP_Bullet.BP_Bullet_C" (Transformation|GetWorldTransform _bulletspawnpoint) "Undefined" "MultiplyWithRoot" 0 _currenttarget self 0))
                (Effects|Components|ParticleSystem|SetFloatParameter (Variables|/Game/_Game/BP/BP_Bullet.BP_Bullet_C|GetNS_Tracer _returnvalue) "BulletSize" 3e+01)
                (Math|Float|IncrementFloat (Variables|InGameStats|GetRoundsFired))))))))))

(event Custom|OverHeatCoolDown
  (bind _towertop (Variables|Default|GetTowerTop))
  (bind _enemiesinrange (Variables|Default|GetEnemiesInRange))
  (bind _relativerotation (Variables|/Script/Engine.SceneComponent|GetRelativeRotation _towertop))
  ;[0.15 0.15 0.15 0.5] Overlap
  (Variables|Default|SetCurrentHeat 0.0)
  (Variables|Default|SetbIsOverheated false)
  (Utilities|FlowControl|Sequence
    (:then_0
      (bind _a (Timeline|Timeline Play)
        (:Update
          (Transformation|SetRelativeRotation _towertop (Math|Rotator|MakeRotator (Math|Float|Lerp -2e+01 0.0 _a) (.pitch _relativerotation) (.yaw _relativerotation)) false false))))
    (:then_1
      (Utilities|FlowControl|DoOnce false
        (:Completed
          (CallFunction|OverheatAnimDeActivete)
          (for _array_element _enemiesinrange
            (Utilities|IsValid _array_element
              (:Is%20Not%20Valid
                (Utilities|Array|RemoveItem _enemiesinrange _array_element))))
          (if (Utilities|Array|IsEmpty _enemiesinrange)
            (Variables|Default|SetbIsTargetingEnemy false)))))
    (:then_2
      (Utilities|FlowControl|DoOnce false) ; enters at Reset
    )))

(event EventBeginPlay
  (bind _towerrange (Variables|Default|GetTowerRange))
  ;[0.15 0.15 0.15 0.5] Beginplay
  (bind _asbp_instance (Utilities|Casting|CastToBP_Instance (Game|GetGameInstance)))
  (Variables|Default|SetAs%20BP%20Instance _asbp_instance)
  (Variables|Default|SetTower self)
  (Rendering|SetVisibility _towerrange false false)
  (Transformation|SetRelativeScale3D (Variables|Default|GetTowerRange) (* (Variables|/Script/Engine.SceneComponent|GetRelativeScale3D (Variables|Default|GetExample)) 8.0))
  (Transformation|SetRelativeScale3D _towerrange (* (Variables|/Script/Engine.SceneComponent|GetRelativeScale3D _towerrange) (.TowerRange (Utilities|Struct|BreakStructure_TowerBase (.BaseTowerStats (Utilities|Struct|BreakStructure_ByteBlaster (Variables|/Game/_Game/BP/Frameworks/BP_Instance.BP_Instance_C|GetByteStats (Variables|Default|GetAs%20BP%20Instance)))))) 0.9))
  (|CallParentFunction))

(event EventUpdateInstalled
  (params (UpdatePrice :type Integer))
  ;[0.15 0.15 0.15 0.5] Interface
  (|CallParentFunction UpdatePrice))

(event EventTick
  (params (DeltaSeconds :type Float%20%28single-precision%29))
  ;[0.15 0.15 0.15 0.5] Tick
  (|CallParentFunction DeltaSeconds))

(event EventEnemyDied
  (params (DropMoney :type Float%20%28double-precision%29))
  (bind _returnvalue (Game|Player|GetPlayerPawn 0))
  ;[0.15 0.15 0.15 0.5] Interface
  (Variables|InGameStats|SetTotalCreditEarned (+ DropMoney (Variables|InGameStats|GetTotalCreditEarned)))
  (bind _money (Class|BPIGeneral|GetMoney(Message) _returnvalue))
  (Class|BPIGeneral|MoneyChanged(Message) _returnvalue (Math|Float|Truncate (+ _money DropMoney))))

(event EventBulletHit
  (params (HittedEnemy :type Actor%20Object%20Reference) (Damage :type Float%20%28double-precision%29) (bIsCrit :type Boolean))
  (bind _enemiesinrange (Variables|Default|GetEnemiesInRange))
  (bind _currenttarget (Variables|Default|GetCurrentTarget))
  (bind _as_bp_instance (Variables|Default|GetAs%20BP%20Instance))
  (bind _as_bp_instance_2 (Variables|Default|GetAs%20BP%20Instance))
  (bind _currenttarget_2 (Variables|Default|GetCurrentTarget))
  (bind _bytestats (Variables|/Game/_Game/BP/Frameworks/BP_Instance.BP_Instance_C|GetByteStats _as_bp_instance))
  (bind _bytestats_2 (Variables|/Game/_Game/BP/Frameworks/BP_Instance.BP_Instance_C|GetByteStats _as_bp_instance_2))
  (bind (_basetowerstats _towerdamage _towerspeed) (Utilities|Struct|BreakStructure_ByteBlaster _bytestats))
  (bind (_basetowerstats_2 _towerdamage_2 _towerspeed_2 _towercritchance _towercritmultiplier) (Utilities|Struct|BreakStructure_ByteBlaster _bytestats_2))
  (bind _returnvalue (* _towerdamage _towercritmultiplier))
  ;[0.15 0.15 0.15 0.5] Overlap
  (if (<= (* _towercritchance 1e+02) (Math|Random|RandomFloatinRange 0.0 1e+02))
    (|CallParentFunction HittedEnemy _towerdamage false)
    (Variables|InGameStats|SetTotalDamage (+ _towerdamage (Variables|InGameStats|GetTotalDamage)))
    (bind (_currenthealth _maxhealth) (Class|BPIEnemy|GetEnemyHealth(Message) _currenttarget_2))
    (Class|BPIEnemy|SetHealth(Message) _currenttarget_2 (- _currenthealth _towerdamage) _maxhealth)
    (else
      (|CallParentFunction HittedEnemy _returnvalue true)
      (Math|Float|IncrementFloat (Variables|InGameStats|GetTotalCritcHit)
        (:%20%20
          (Variables|InGameStats|SetTotalDamage (+ (Variables|InGameStats|GetTotalDamage) _returnvalue))
          (bind (_currenthealth_2 _maxhealth_2) (Class|BPIEnemy|GetEnemyHealth(Message) _currenttarget_2))
          (Class|BPIEnemy|SetHealth(Message) _currenttarget_2 (- _currenthealth_2 _returnvalue) _maxhealth_2)))))
  (bind _currenthealth_3 (Class|BPIEnemy|GetEnemyHealth(Message) _currenttarget_2))
  (if (<= _currenthealth_3 0.0)
    (Utilities|Array|RemoveItem _enemiesinrange _currenttarget)
    (if (Utilities|Array|IsEmpty _enemiesinrange)
      (Variables|Default|SetbIsTargetingEnemy false))
    (Class|BPIEnemy|EnemyKilled(Message) _currenttarget self)))

(fn ConstructionScript
  (|CallParentFunction))

(fn OverheatAnimActivete
  (|CallParentFunction))

(fn OverheatAnimDeActivete
  (|CallParentFunction))

(fn GetTowerStats
  (return (Variables|InGameStats|GetTotalDamage) (Variables|InGameStats|GetRoundsFired) (Variables|InGameStats|GetTotalCritcHit) (Variables|InGameStats|GetOverheatCount) (Variables|InGameStats|GetTotalCreditEarned) (Variables|Default|GetTowerSellPrice) (Variables|Default|GetCurrentHeat) 0.0 0.0 0.0 0.0))