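; BP_GhostSupport is the ghost variant of the support tower, identifying itself by returning true from GetIsGhostTower.
; On BeginPlay it caches the BP_Instance game instance and sizes TowerRange from the Example component's scale.
; It enlarges that range further only when the support tower's range stat in the game instance exactly equals a specific value.
; Construction defers entirely to the parent class.
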(event EventBeginPlay
  (bind _towerrange (Variables|Default|GetTowerRange))
  (bind _asbp_instance (Utilities|Casting|CastToBP_Instance (Game|GetGameInstance)))
  (Variables|Default|SetAs%20BP%20Instance _asbp_instance)
  (Transformation|SetRelativeScale3D (Variables|Default|GetTowerRange) (* (Variables|/Script/Engine.SceneComponent|GetRelativeScale3D (Variables|Default|GetExample)) 8.0))
  (if (== (.TowerRange (Utilities|Struct|BreakStructure_TowerBase (.BaseTowerStats (Utilities|Struct|BreakStructure_BoostServer (Variables|/Game/_Game/BP/Frameworks/BP_Instance.BP_Instance_C|GetSupportStats (Variables|Default|GetAs%20BP%20Instance)))))) 2.0)
    (Transformation|SetRelativeScale3D _towerrange (* (Variables|/Script/Engine.SceneComponent|GetRelativeScale3D _towerrange) (.TowerRange (Utilities|Struct|BreakStructure_TowerBase (.BaseTowerStats (Utilities|Struct|BreakStructure_BoostServer (Variables|/Game/_Game/BP/Frameworks/BP_Instance.BP_Instance_C|GetSupportStats (Variables|Default|GetAs%20BP%20Instance)))))) 0.85))))

(fn ConstructionScript
  (|CallParentFunction))

(fn GetIsGhostTower
  (return true))