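; BP_GhostSurge is a Ghost tower Blueprint for the Surge stats entry, extending a parent tower class.
; On BeginPlay it caches the BP_Instance game instance and scales its Plane23 mesh by the Surge tower range times 0.9, presumably sizing a range indicator for the placement preview.
; The construction script only runs the parent's.
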(event EventBeginPlay
  (bind _plane23 (Variables|Default|GetPlane23))
  (bind _asbp_instance (Utilities|Casting|CastToBP_Instance (Game|GetGameInstance)))
  (Variables|Default|SetAs%20BP%20Instance _asbp_instance)
  (Transformation|SetRelativeScale3D _plane23 (* (Variables|/Script/Engine.SceneComponent|GetRelativeScale3D _plane23) (.TowerRange (Utilities|Struct|BreakStructure_TowerBase (.BaseTowerStats (Utilities|Struct|BreakStructure_SurgeTower (Variables|/Game/_Game/BP/Frameworks/BP_Instance.BP_Instance_C|GetSurgeStats (Variables|Default|GetAs%20BP%20Instance)))))) 0.9)))

(fn ConstructionScript
  (|CallParentFunction))