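; BP_TowerSupport is a support tower that reports boost, assist and buff totals through the shared tower stats output.
; BeginPlay sizes and hides its range, then starts a looping timer that spins the tower top.
; Installing an update calls the parent, enables OverheatPass and records an install round.
; Box overlaps with other towers only print their names; no buff logic appears here.
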(event OnComponentBeginOverlap(Box)
  (params (OverlappedComponent :type Primitive%20Component%20Object%20Reference) (OtherActor :type Actor%20Object%20Reference) (OtherComp :type Primitive%20Component%20Object%20Reference) (OtherBodyIndex :type Integer) (bFromSweep :type Boolean) (SweepResult :type Hit%20Result%20Structure%20%28by%20ref%29))
  ;[0.15 0.15 0.15 0.5] Beginplay
  (if (and (Utilities|DoesObjectImplementInterface OtherActor "/Game/_Game/BP/Frameworks/BPI_Towers.BPI_Towers_C") (!= OtherActor self))
    (Development|PrintString (Utilities|GetDisplayName OtherActor) true true "(R=1.000000,G=0.000000,B=0.649983,A=1.000000)" 4.0)))

(event Custom|Spin
  ;[0.15 0.15 0.15 0.5] Beginplay
  (Transformation|AddLocalRotation (Variables|Default|GetTowerTopSupport) (Math|Rotator|MakeRotator 0.0 0.0 (* (Utilities|Time|GetWorldDeltaSeconds) 5.1e+02)) false false))

(event EventBeginPlay
  ;[0.15 0.15 0.15 0.5] Beginplay
  (Variables|Default|SetTower self)
  (Rendering|SetVisibility (Variables|Default|GetTowerRange) false false)
  (Transformation|SetRelativeScale3D (Variables|Default|GetTowerRange) (* (Variables|/Script/Engine.SceneComponent|GetRelativeScale3D (Variables|Default|GetExample)) 8.0))
  (|CallParentFunction)
  (Utilities|Time|SetTimerbyEvent (delegate Custom|Spin) 0.06 true))

(event EventUpdateInstalled
  (params (UpdatePrice :type Integer) (UpdateNumber :type Integer) (bGecici :type Boolean))
  ;[0.15 0.15 0.15 0.5] Interface
  (|CallParentFunction UpdatePrice UpdateNumber bGecici)
  (Variables|Default|SetOverheatPass true)
  (Variables|Default|SetOverheatInstalledRound (.Update6InstalledRound (Utilities|Struct|BreakStructure_Updates (Variables|Default|GetStructre_Updates)))))

(fn ConstructionScript
  (|CallParentFunction))

(fn GetTowerStats
  (return (Variables|InGameStats|GetTotalDamageBoost) (Variables|InGameStats|GetTotalSpeedBoost) (Variables|InGameStats|GetAssistedCriticalHits) (Variables|InGameStats|GetOverheatCount) 0.0 (Variables|Default|GetTowerSellPrice) (Variables|Default|GetCurrentHeat) (Variables|InGameStats|GetTotalTowerBuffed) 0.0 0.0 0.0))