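; Missile launcher tower for tower defense that fires homing-target rockets at enemies in range, with stats read from the game instance.
; A looping attack timer spawns bullets and builds heat, tilting the top and pausing fire on overheat.
; Hits deal direct damage and sweep a growing sphere for crit-capable splash, periodically enlarged, applying Frost slow or Flame burn.
; Six upgrades adjust income, targeting flags and round-limited damage, speed or overheat immunity.
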(event OnComponentBeginOverlap(Box)
  (params (OverlappedComponent :type Primitive%20Component%20Object%20Reference) (OtherActor :type Actor%20Object%20Reference) (OtherComp :type Primitive%20Component%20Object%20Reference) (OtherBodyIndex :type Integer) (bFromSweep :type Boolean) (SweepResult :type Hit%20Result%20Structure%20%28by%20ref%29))
  ;[0.15 0.15 0.15 0.5] Overlap
  (if (Utilities|DoesObjectImplementInterface OtherActor "/Game/_Game/BP/Frameworks/BPI_Enemy.BPI_Enemy_C")
    (Utilities|Array|Add (Variables|Default|GetEnemiesInRange) OtherActor)
    (if (Variables|Default|GetbIsTargetingEnemy)
      _
      (else
        (Variables|Default|SetbIsTargetingEnemy true)))
    (if (not (Utilities|Time|IsTimerActivebyHandle (Variables|Default|GetAttackTimerHandle)))
      (bind _returnvalue (Utilities|Time|SetTimerbyEvent (delegate Custom|AttackToEnemy) (* (.TowerSpeed (Utilities|Struct|BreakStructure_MissleLauncher (Variables|/Game/_Game/BP/Frameworks/BP_Instance.BP_Instance_C|GetMissleStats (Variables|Default|GetAs%20BP%20Instance)))) (Variables|Default|GetSpeedMultiplier)) true))
      (Variables|Default|SetAttackTimerHandle _returnvalue))))

(event OnComponentEndOverlap(Box)
  (params (OverlappedComponent :type Primitive%20Component%20Object%20Reference) (OtherActor :type Actor%20Object%20Reference) (OtherComp :type Primitive%20Component%20Object%20Reference) (OtherBodyIndex :type Integer))
  (bind _enemiesinrange (Variables|Default|GetEnemiesInRange))
  ;[0.15 0.15 0.15 0.5] Overlap
  (if (Utilities|DoesObjectImplementInterface OtherActor "/Game/_Game/BP/Frameworks/BPI_Enemy.BPI_Enemy_C")
    (Utilities|Array|RemoveItem _enemiesinrange OtherActor)
    (if (== OtherActor (Variables|Default|GetCurrentTarget))
      (CallFunction|SelectTarget)
      (if (Utilities|Array|IsEmpty _enemiesinrange)
        (Variables|Default|SetbIsTargetingEnemy false)))))

(event OnComponentBeginOverlap(SphereAoE)
  (params (OverlappedComponent :type Primitive%20Component%20Object%20Reference) (OtherActor :type Actor%20Object%20Reference) (OtherComp :type Primitive%20Component%20Object%20Reference) (OtherBodyIndex :type Integer) (bFromSweep :type Boolean) (SweepResult :type Hit%20Result%20Structure%20%28by%20ref%29))
  (bind _enemiesinrange (Variables|Default|GetEnemiesInRange))
  (bind _as_bp_instance (Variables|Default|GetAs%20BP%20Instance))
  (bind _damagemultiplier (Variables|Default|GetDamageMultiplier))
  (bind _bigrocketdamagemultiplier (Variables|Default|GetBigRocketDamageMultiplier))
  (bind _misslestats (Variables|/Game/_Game/BP/Frameworks/BP_Instance.BP_Instance_C|GetMissleStats _as_bp_instance))
  (bind (_basetowerstats _towerdamage _towerspeed _towercritchance _towercritmultiplier) (Utilities|Struct|BreakStructure_MissleLauncher _misslestats))
  (bind _returnvalue (* _towerdamage _damagemultiplier _bigrocketdamagemultiplier))
  (bind _returnvalue_2 (* _returnvalue _towercritmultiplier))
  ;[0.15 0.15 0.15 0.5] Overlap
  (if (and (not (Utilities|Array|ContainsItem (Variables|Default|GetHitEnemies) 0)) (Utilities|DoesObjectImplementInterface OtherActor "/Game/_Game/BP/Frameworks/BPI_Enemy.BPI_Enemy_C"))
    (Utilities|IsValid OtherActor
      (:Is%20Valid
        (Utilities|Array|Add (Variables|Default|GetHitEnemies) OtherActor)
        (if (<= (* _towercritchance 1e+02) (Math|Random|RandomFloatinRange 0.0 1e+02))
          (Variables|InGameStats|SetTotalDamageDealt (+ (Variables|InGameStats|GetTotalDamageDealt) _returnvalue))
          (Variables|InGameStats|SetTotalAoE (+ (Variables|InGameStats|GetTotalAoE) _returnvalue))
          (bind (_currenthealth _maxhealth) (Class|BPIEnemy|GetEnemyHealth(Message) OtherActor))
          (Class|BPIEnemy|SetHealth(Message) OtherActor (- _currenthealth _returnvalue) _maxhealth)
          (CallFunction|EnemyTakeDamage OtherActor)
          (Utilities|IsValid OtherActor
            (:Is%20Valid
              (Game|SpawnActorfromClass "/Game/_Game/BP/BP_DamageText.BP_DamageText_C" (Math|Transform|MakeTransform (+ (Transformation|GetActorLocation OtherActor) "0.000000,0.000000,120.000000") "0, 0, 0" "1.000000,1.000000,1.000000") "Undefined" "MultiplyWithRoot" 0 _returnvalue false 0)))
          (else
            (Math|Float|IncrementFloat (Variables|InGameStats|GetTotalCritHit)
              (:%20%20
                (Variables|InGameStats|SetTotalDamageDealt (+ (Variables|InGameStats|GetTotalDamageDealt) _returnvalue_2))
                (Variables|InGameStats|SetTotalAoE (+ (Variables|InGameStats|GetTotalAoE) _returnvalue_2))
                (bind (_currenthealth_2 _maxhealth_2) (Class|BPIEnemy|GetEnemyHealth(Message) OtherActor))
                (Class|BPIEnemy|SetHealth(Message) OtherActor (- _currenthealth_2 _returnvalue_2) _maxhealth_2)
                (CallFunction|EnemyTakeDamage OtherActor)
                (Utilities|IsValid OtherActor
                  (:Is%20Valid
                    (Game|SpawnActorfromClass "/Game/_Game/BP/BP_DamageText.BP_DamageText_C" (Math|Transform|MakeTransform (+ (Transformation|GetActorLocation OtherActor) "0.000000,0.000000,120.000000") "0, 0, 0" "1.000000,1.000000,1.000000") "Undefined" "MultiplyWithRoot" 0 _returnvalue_2 true 0)))))))
        (bind _currenthealth_3 (Class|BPIEnemy|GetEnemyHealth(Message) OtherActor))
        (Class|BPIEnemy|EnemyDamageTaken(Message) OtherActor)
        (if (<= _currenthealth_3 0.0)
          (Utilities|Array|RemoveItem _enemiesinrange OtherActor)
          (if (Utilities|Array|IsEmpty _enemiesinrange)
            (Variables|Default|SetbIsTargetingEnemy false))
          (Class|BPIEnemy|EnemyKilled(Message) OtherActor self))))))

(event Custom|AttackToEnemy
  (bind _as_bp_instance (Variables|Default|GetAs%20BP%20Instance))
  (bind _towertop (Variables|Default|GetTowerTop))
  (bind _enemiesinrange (Variables|Default|GetEnemiesInRange))
  (bind _currenttarget (Variables|Default|GetCurrentTarget))
  (bind _bulletspawnpoint (Variables|Default|GetBulletSpawnPoint))
  (bind _relativerotation (Variables|/Script/Engine.SceneComponent|GetRelativeRotation _towertop))
  (bind _misslestats (Variables|/Game/_Game/BP/Frameworks/BP_Instance.BP_Instance_C|GetMissleStats _as_bp_instance))
  (bind (_basetowerstats _towerdamage _towerspeed) (Utilities|Struct|BreakStructure_MissleLauncher _misslestats))
  (bind (_towerrange _toweroverheattime _toweroverheatduration) (Utilities|Struct|BreakStructure_TowerBase _basetowerstats))
  ;[0.15 0.15 0.15 0.5] Overlap
  (Utilities|FlowControl|Sequence
    (:then_0
      (if (and (or (Variables|Default|GetbIsOverheated) (not (Variables|Default|GetbIsTargetingEnemy))) (and (> (Variables|Default|GetCurrentHeat) 0.0) (< (Variables|Default|GetCurrentHeat) _toweroverheattime)))
        (Variables|Default|SetCurrentHeat (- (Variables|Default|GetCurrentHeat) _towerspeed))))
    (:then_1
      (if (and (Variables|Default|GetbIsTargetingEnemy) (not (Variables|Default|GetbIsOverheated)))
        (Utilities|FlowControl|Sequence
          (:then_0
            (if (Variables|Default|GetbIsTargetingEnemy)
              (if (not (and (Variables|Default|GetOverheatPass) (== (Variables|Default|GetFinished%20Round) (Variables|Default|GetOverheatInstalledRound))))
                (bind _output_get (Variables|Default|SetCurrentHeat (+ _towerspeed (Variables|Default|GetCurrentHeat))))
                (if (>= _output_get _toweroverheattime)
                  (Math|Float|IncrementFloat (Variables|InGameStats|GetOverheatCount)
                    (:%20%20
                      (Variables|Default|SetbIsOverheated true)
                      (Utilities|FlowControl|Sequence
                        (:then_0
                          (bind _a (Timeline|Timeline_0_0 PlayFromStart)
                            (:Update
                              (Transformation|SetRelativeRotation _towertop (Math|Rotator|MakeRotator (Math|Float|Lerp 0.0 -2e+01 _a) (.pitch _relativerotation) (.yaw _relativerotation)) false false))
                            (:Finished
                              (Utilities|FlowControl|DoOnce false) ; enters at Reset
                            )))
                        (:then_1
                          (Utilities|FlowControl|DoOnce false
                            (:Completed
                              (CallFunction|OverheatAnimActivete)
                              (Utilities|Time|SetTimerbyEvent (delegate Custom|OverHeatCoolDown) _toweroverheatduration)))))))))))
          (:then_1
            (Utilities|IsValid _currenttarget
              (:Is%20Valid
                (Niagara|SpawnSystematLocation "/Game/_Game/Niagara/NS_Muzzle.NS_Muzzle" (.location (Transformation|GetWorldTransform _bulletspawnpoint)))
                (bind _returnvalue (Game|SpawnActorfromClass "/Game/_Game/BP/BP_Bullet.BP_Bullet_C" (Transformation|GetWorldTransform _bulletspawnpoint) "Undefined" "MultiplyWithRoot" 0 _currenttarget self 0))
                (Effects|Components|ParticleSystem|SetFloatParameter (Variables|/Game/_Game/BP/BP_Bullet.BP_Bullet_C|GetNS_Tracer _returnvalue) "BulletSize" 6e+01)))))))))

(event Custom|OverHeatCoolDown
  (bind _towertop (Variables|Default|GetTowerTop))
  (bind _enemiesinrange (Variables|Default|GetEnemiesInRange))
  (bind _relativerotation (Variables|/Script/Engine.SceneComponent|GetRelativeRotation _towertop))
  ;[0.15 0.15 0.15 0.5] Overlap
  (Variables|Default|SetCurrentHeat 0.0)
  (Variables|Default|SetbIsOverheated false)
  (Utilities|FlowControl|Sequence
    (:then_0
      (bind _a (Timeline|Timeline_1 Play)
        (:Update
          (Transformation|SetRelativeRotation _towertop (Math|Rotator|MakeRotator (Math|Float|Lerp -2e+01 0.0 _a) (.pitch _relativerotation) (.yaw _relativerotation)) false false))))
    (:then_1
      (Utilities|FlowControl|DoOnce false
        (:Completed
          (CallFunction|OverheatAnimDeActivete)
          (for _array_element _enemiesinrange
            (Utilities|IsValid _array_element
              (:Is%20Not%20Valid
                (Utilities|Array|RemoveItem _enemiesinrange _array_element))))
          (if (Utilities|Array|IsEmpty _enemiesinrange)
            (Variables|Default|SetbIsTargetingEnemy false)))))
    (:then_2
      (Utilities|FlowControl|DoOnce false) ; enters at Reset
    )))

(event Custom|EnemyTakeDamage
  (params (Enemy :type Actor%20Object%20Reference))
  ;[0.15 0.15 0.15 0.5] EnemyEffects
  (switch string (Variables|Default|GetTower%20Rocket%20Type)
    (:Frost
      (Utilities|IsValid Enemy
        (:Is%20Valid
          (Class|BPIEnemy|EnemyEffect(Message) Enemy "Slow" self 0.0 0.0 (Variables|Default|GetTower%20Special%20Skill%20Slow%20Enemies%20Duration) (Variables|Default|GetTower%20Special%20Skill%20Slow%20Enemies)))))
    (:Flame
      (Utilities|IsValid Enemy
        (:Is%20Valid
          (Class|BPIEnemy|EnemyEffect(Message) Enemy "Fire" self (Variables|Default|GetTower%20Special%20Skill%20Flame%20Enemies) (Variables|Default|GetTower%20Special%20Skill%20Flame%20Enemies%20Duration) 0.0 0.0))))))

(event EventBeginPlay
  (bind _towerrange (Variables|Default|GetTowerRange))
  ;[0.15 0.15 0.15 0.5] Beginplay
  (bind _asbp_instance (Utilities|Casting|CastToBP_Instance (Game|GetGameInstance)))
  (Variables|Default|SetAs%20BP%20Instance _asbp_instance)
  (Variables|Default|SetTower self)
  (Rendering|SetVisibility _towerrange false false)
  (Transformation|SetRelativeScale3D (Variables|Default|GetTowerRange) (* (Variables|/Script/Engine.SceneComponent|GetRelativeScale3D (Variables|Default|GetExample)) 8.0))
  (Transformation|SetRelativeScale3D _towerrange (* (Variables|/Script/Engine.SceneComponent|GetRelativeScale3D _towerrange) (.TowerRange (Utilities|Struct|BreakStructure_TowerBase (.BaseTowerStats (Utilities|Struct|BreakStructure_MissleLauncher (Variables|/Game/_Game/BP/Frameworks/BP_Instance.BP_Instance_C|GetMissleStats (Variables|Default|GetAs%20BP%20Instance)))))) 0.82))
  (Variables|Default|SetTower%20Special%20Skill%20Mega%20Rocket (.TowerSpecialSkillMegaRocket (Utilities|Struct|BreakStructure_MissleLauncher (Variables|/Game/_Game/BP/Frameworks/BP_Instance.BP_Instance_C|GetMissleStats (Variables|Default|GetAs%20BP%20Instance)))))
  (Variables|Default|SetTower%20Special%20Skill%20Slow%20Enemies (.TowerSpecialSkillSlowEnemies (Utilities|Struct|BreakStructure_MissleLauncher (Variables|/Game/_Game/BP/Frameworks/BP_Instance.BP_Instance_C|GetMissleStats (Variables|Default|GetAs%20BP%20Instance)))))
  (Variables|Default|SetTower%20Special%20Skill%20Slow%20Enemies%20Duration (.TowerSpecialSkillSlowEnemiesDuration (Utilities|Struct|BreakStructure_MissleLauncher (Variables|/Game/_Game/BP/Frameworks/BP_Instance.BP_Instance_C|GetMissleStats (Variables|Default|GetAs%20BP%20Instance)))))
  (Variables|Default|SetTower%20Special%20Skill%20Flame%20Enemies (.TowerSpecialSkillFlameEnemies (Utilities|Struct|BreakStructure_MissleLauncher (Variables|/Game/_Game/BP/Frameworks/BP_Instance.BP_Instance_C|GetMissleStats (Variables|Default|GetAs%20BP%20Instance)))))
  (Variables|Default|SetTower%20Special%20Skill%20Flame%20Enemies%20Duration (.TowerSpecialSkillFlameEnemiesDuration (Utilities|Struct|BreakStructure_MissleLauncher (Variables|/Game/_Game/BP/Frameworks/BP_Instance.BP_Instance_C|GetMissleStats (Variables|Default|GetAs%20BP%20Instance)))))
  (Variables|Default|SetTower%20Rocket%20Type (.TowerRocketType (Utilities|Struct|BreakStructure_MissleLauncher (Variables|/Game/_Game/BP/Frameworks/BP_Instance.BP_Instance_C|GetMissleStats (Variables|Default|GetAs%20BP%20Instance)))))
  (|CallParentFunction))

(event EventUpdateInstalled
  (params (UpdatePrice :type Integer) (UpdateNumber :type Integer) (bGecici :type Boolean))
  ;[0.15 0.15 0.15 0.5] Interface
  (|CallParentFunction UpdatePrice UpdateNumber bGecici)
  (Utilities|MUpdate UpdateNumber bGecici))

(event EventTick
  (params (DeltaSeconds :type Float%20%28single-precision%29))
  ;[0.15 0.15 0.15 0.5] Tick
  (|CallParentFunction DeltaSeconds))

(event EventEnemyDied
  (params (DropMoney :type Float%20%28double-precision%29))
  (bind _returnvalue (Game|Player|GetPlayerPawn 0))
  (bind _moneymultiplier (Variables|Default|GetMoneyMultiplier))
  (bind _returnvalue_2 (* DropMoney _moneymultiplier))
  ;[0.15 0.15 0.15 0.5] Interface
  (Variables|InGameStats|SetTotalCreditEarned (+ _returnvalue_2 (Variables|InGameStats|GetTotalCreditEarned)))
  (bind _money (Class|BPIGeneral|GetMoney(Message) _returnvalue))
  (Class|BPIGeneral|MoneyChanged(Message) _returnvalue (Math|Float|Truncate (+ _money _returnvalue_2))))

(event EventEnemyTakeFireDamage
  (params (Enemy :type Actor%20Object%20Reference) (EnemyHealth :type Float%20%28double-precision%29))
  (bind _enemiesinrange (Variables|Default|GetEnemiesInRange))
  ;[0.15 0.15 0.15 0.5] EnemyEffects
  (Variables|InGameStats|SetTotalDamageDealt (+ (Variables|InGameStats|GetTotalDamageDealt) (Variables|Default|GetTower%20Special%20Skill%20Flame%20Enemies)))
  (bind _currenthealth (Class|BPIEnemy|GetEnemyHealth(Message) Enemy))
  (Class|BPIEnemy|EnemyDamageTaken(Message) Enemy)
  (if (<= _currenthealth 0.0)
    (Utilities|Array|RemoveItem _enemiesinrange Enemy)
    (if (Utilities|Array|IsEmpty _enemiesinrange)
      (Variables|Default|SetbIsTargetingEnemy false))
    (Class|BPIEnemy|EnemyKilled(Message) Enemy self)))

(event EventRoundEndedTowers
  (params (FinishedRound :type Float%20%28double-precision%29))
  ;[0.15 0.15 0.15 0.5] Interface
  (bind _output_get (Variables|Default|SetFinished%20Round FinishedRound))
  (Utilities|FlowControl|Sequence
    (:then_0
      (if (== (- _output_get (Variables|Default|GetDamagenstalledRound)) 1.0)
        (Variables|Default|SetDamageMultiplier 1.0)))
    (:then_1
      (if (== (- _output_get (Variables|Default|GetSpeednstalledRound)) 1.0)
        (Variables|Default|SetSpeedMultiplier 1.0)))))

(event EventBulletHit
  (params (HittedEnemy :type Actor%20Object%20Reference) (Damage :type Float%20%28double-precision%29) (bIsCrit :type Boolean))
  (bind _sphereaoe (Variables|Default|GetSphereAoE))
  (bind _p_lightning_02_big (Variables|Default|GetP_Lightning_02_Big))
  (bind _as_bp_instance (Variables|Default|GetAs%20BP%20Instance))
  (bind _damagemultiplier (Variables|Default|GetDamageMultiplier))
  (bind _enemiesinrange (Variables|Default|GetEnemiesInRange))
  (bind _misslestats (Variables|/Game/_Game/BP/Frameworks/BP_Instance.BP_Instance_C|GetMissleStats _as_bp_instance))
  (bind (_basetowerstats _towerdamage _towerspeed _towercritchance _towercritmultiplier) (Utilities|Struct|BreakStructure_MissleLauncher _misslestats))
  (bind _returnvalue (* _towerdamage _damagemultiplier))
  (bind _returnvalue_2 (* _returnvalue _towercritmultiplier))
  ;[0.15 0.15 0.15 0.5] Overlap
  (bind _result (Math|Integer|IncrementInt (Variables|Default|GetRocketCount))
    (:%20%20
      (if (== _result 5)
        (Variables|Default|SetRocketCount 0)
        (Variables|Default|SetBigRocketDamageMultiplier 1.5)
        (Variables|Default|SetBigRocketRadiusMultiplier 1.5)
        (else
          (Variables|Default|SetBigRocketDamageMultiplier 1.0)
          (Variables|Default|SetBigRocketRadiusMultiplier 1.0)))
      (Utilities|FlowControl|Sequence
        (:then_0
          (bind _output_get (Variables|Default|SetExplotionRadius (Transformation|GetActorLocation HittedEnemy)))
          (Transformation|SetWorldLocation (Variables|Default|GetSphereAoE) _output_get false false)
          (Transformation|SetWorldLocation _p_lightning_02_big _output_get false false)
          (Rendering|SetVisibility _p_lightning_02_big true false)
          (bind _returnvalue_3 (Niagara|SpawnSystematLocation "/Game/_Game/Niagara/NS_RocketExplosion.NS_RocketExplosion" _output_get))
          (Effects|Components|ParticleSystem|SetFloatParameter _returnvalue_3 "User.ExplotionRadius" (/ (* (.x (.BoxExtent (Collision|GetComponentBounds (Variables|Default|GetExample)))) (.TowerHitAreaLenght (Utilities|Struct|BreakStructure_MissleLauncher (Variables|/Game/_Game/BP/Frameworks/BP_Instance.BP_Instance_C|GetMissleStats (Variables|Default|GetAs%20BP%20Instance)))) (Variables|Default|GetBigRocketRadiusMultiplier)) 15.0))
          (switch string (Variables|Default|GetTower%20Rocket%20Type)
            (:Normal
              (Niagara|SetNiagaraVariable(LinearColor) _returnvalue_3 "User.Color" (Utilities|Struct|MakeLinearColor 0.023308 0.168993 0.348958 1.0))
              (bind _alpha (Timeline|Timeline PlayFromStart)
                (:Update
                  (Components|Sphere|SetSphereRadius _sphereaoe (Math|Float|Lerp 0.0 (* (.x (.BoxExtent (Collision|GetComponentBounds (Variables|Default|GetExample)))) (.TowerHitAreaLenght (Utilities|Struct|BreakStructure_MissleLauncher (Variables|/Game/_Game/BP/Frameworks/BP_Instance.BP_Instance_C|GetMissleStats (Variables|Default|GetAs%20BP%20Instance)))) (Variables|Default|GetBigRocketRadiusMultiplier)) _alpha) true))
                (:Finished
                  (Components|Sphere|SetSphereRadius _sphereaoe 0.0 true)
                  (Rendering|SetVisibility _p_lightning_02_big false false)
                  (Transformation|SetWorldLocation _sphereaoe (Transformation|GetActorLocation) false false)
                  (Components|DestroyComponent _returnvalue_3)
                  (Utilities|Array|Clear (Variables|Default|GetHitEnemies)))))
            (:Frost
              (Niagara|SetNiagaraVariable(LinearColor) _returnvalue_3 "User.Color" (Utilities|Struct|MakeLinearColor 0.5 0.8 1.0 1.0))
              (Timeline|Timeline PlayFromStart))
            (:Flame
              (Niagara|SetNiagaraVariable(LinearColor) _returnvalue_3 "User.Color" (Utilities|Struct|MakeLinearColor 0.421875 0.210066 0.0 1.0))
              (Timeline|Timeline PlayFromStart))))
        (:then_1
          (if (<= (* _towercritchance 1e+02) (Math|Random|RandomFloatinRange 0.0 1e+02))
            (Utilities|IsValid HittedEnemy
              (:Is%20Valid
                (|CallParentFunction HittedEnemy _returnvalue false)
                (Variables|InGameStats|SetTotalDamageDealt (+ (Variables|InGameStats|GetTotalDamageDealt) _returnvalue))
                (bind (_currenthealth _maxhealth) (Class|BPIEnemy|GetEnemyHealth(Message) HittedEnemy))
                (Class|BPIEnemy|SetHealth(Message) HittedEnemy (- _currenthealth _returnvalue) _maxhealth)))
            (else
              (Utilities|IsValid HittedEnemy
                (:Is%20Valid
                  (|CallParentFunction HittedEnemy _returnvalue_2 false)
                  (Math|Float|IncrementFloat (Variables|InGameStats|GetTotalCritHit)
                    (:%20%20
                      (Variables|InGameStats|SetTotalDamageDealt (+ (Variables|InGameStats|GetTotalDamageDealt) _returnvalue_2))
                      (bind (_currenthealth_2 _maxhealth_2) (Class|BPIEnemy|GetEnemyHealth(Message) HittedEnemy))
                      (Class|BPIEnemy|SetHealth(Message) HittedEnemy (- _currenthealth_2 _returnvalue_2) _maxhealth_2)))))))
          (bind _currenthealth_3 (Class|BPIEnemy|GetEnemyHealth(Message) HittedEnemy))
          (Class|BPIEnemy|EnemyDamageTaken(Message) HittedEnemy)
          (if (<= _currenthealth_3 0.0)
            (Utilities|Array|RemoveItem _enemiesinrange HittedEnemy)
            (if (Utilities|Array|IsEmpty _enemiesinrange)
              (Variables|Default|SetbIsTargetingEnemy false))
            (Class|BPIEnemy|EnemyKilled(Message) HittedEnemy self)))))))

(fn ConstructionScript
  (|CallParentFunction))

(fn OverheatAnimActivete
  (|CallParentFunction))

(fn OverheatAnimDeActivete
  (|CallParentFunction))

(fn GetTowerStats
  (return (Variables|InGameStats|GetTotalDamageDealt) 0.0 (Variables|InGameStats|GetTotalCritHit) (Variables|InGameStats|GetOverheatCount) (Variables|InGameStats|GetTotalCreditEarned) (Variables|Default|GetTowerSellPrice) (Variables|Default|GetCurrentHeat) 0.0 0.0 0.0 (Variables|InGameStats|GetTotalAoE)))