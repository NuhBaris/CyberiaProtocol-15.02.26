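; Level-select tower pawn that hops between ten hardcoded level positions as GoForward and GoBack step StandingLevel.
; A shared timeline arcs and pitches the actor while turning TowerTop toward the target, and IsAnimFinished blocks overlapping moves.
; Forward moves are capped by the game instance's CurrentLevel; locked attempts call a warning and play a nudge-and-spin.
; SetLevel sends each level's name, number and reward text to the BP_Computer widget.
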(event Custom|GoForward
  (if (and (Variables|Default|GetbIsAnimFinished) (< (Variables|Default|GetStandingLevel) 10))
    (Variables|Default|SetbMoveModeForward true)
    (CallFunction|JumpTower)))

(event Custom|GoBack
  (if (Variables|Default|GetbIsAnimFinished)
    (Variables|Default|SetbMoveModeForward false)
    (CallFunction|JumpTower)))

(event Custom|JumpTower
  (bind _standinglevel (Variables|Default|GetStandingLevel))
  (bind _standinglevel_2 (Variables|Default|GetStandingLevel))
  (if (Variables|Default|GetbMoveModeForward)
    (if (> (Variables|/Game/_Game/BP/Frameworks/BP_Instance.BP_Instance_C|GetCurrentLevel (Variables|Default|GetAs%20BP%20Instance)) _standinglevel)
      (Math|Integer|IncrementInt _standinglevel
        (:%20%20
          (Variables|Default|SetChangedRotValue 1e+01)
          (Variables|Default|SetbIsAnimFinished false :!label _label)
          (Variables|Default|SetRot (Transformation|GetWorldRotation (Variables|Default|GetTowerTop)))
          (Variables|Default|SetLoc (Transformation|GetActorLocation))
          (Utilities|FlowControl|Sequence
            (:then_0
              (switch int _standinglevel
                (:1
                  (Utilities|SetLevel "Cold Boot" "Reward :  
   - Boost Server" 1))
                (:2
                  (Utilities|SetLevel "Firewall Breach" "Reward :  
     - Laser Curtain" 2))
                (:3
                  (Utilities|SetLevel "Corrupted Files" "Reward :  
     - Surge Tower" 3))
                (:4
                  (Utilities|SetLevel "Network Intrusion" "Reward :  
     - Bullet Time" 4))
                (:5
                  (Utilities|SetLevel "System Overload" "Reward :  
     - Missle Launcher" 5))
                (:6
                  (Utilities|SetLevel "Malware Outbreak" "" 6))
                (:7
                  (Utilities|SetLevel "Core Infection" "Reward :  
     - Thermal Control" 7))
                (:8
                  (Utilities|SetLevel "Data Collapse" "" 8))
                (:9
                  (Utilities|SetLevel "Kernel Panic" "" 9))
                (:10
                  (Utilities|SetLevel "Blink Gone" "" 10))))
            (:then_1
              (switch int _standinglevel
                (:1
                  (Variables|Default|SetNextLoc "71999.846783,3052.340942,1800.000000")
                  (bind (_direction _lineara _upa _rotatea) (Timeline|Timeline PlayFromStart)
                    (:Update
                      (Transformation|SetActorLocation (Math|Vector|MakeVector (Math|Float|Lerp (.X (Math|Vector|BreakVector (Variables|Default|GetLoc))) (.x (Variables|Default|GetNextLoc)) _lineara) (Math|Float|Lerp (.Y (Math|Vector|BreakVector (Variables|Default|GetLoc))) (.y (Variables|Default|GetNextLoc)) _lineara) (Math|Float|Lerp 3648.822499 11103.447169 _upa)) false false)
                      (Transformation|SetActorRotation (Math|Rotator|MakeRotator 0.0 (Math|Float|Lerp 0.0 (Variables|Default|GetChangedRotValue) _upa) 0.0))
                      (Transformation|SetWorldRotation (Variables|Default|GetTowerTop) (Math|Rotator|MakeRotator 0.0 0.0 (Math|Float|Lerp (.yaw (Variables|Default|GetRot)) (+ (.yaw (Math|Rotator|FindLookatRotation (Variables|Default|GetLoc) (Variables|Default|GetNextLoc))) 9e+01) _rotatea)) false false))
                    (:Finished
                      (Variables|Default|SetbIsAnimFinished true))))
                (:2
                  (Variables|Default|SetNextLoc "80036.892070,5390.871417,1800.000000")
                  (Timeline|Timeline PlayFromStart))
                (:3
                  (Variables|Default|SetNextLoc "87960.413323,-1424.041456,1800.000000")
                  (Timeline|Timeline PlayFromStart))
                (:4
                  (Variables|Default|SetNextLoc "95828.826563,6833.115407,1850.000000")
                  (Timeline|Timeline PlayFromStart))
                (:5
                  (Variables|Default|SetNextLoc "103137.477201,3004.297284,1800.000000")
                  (Timeline|Timeline PlayFromStart))
                (:6
                  (Variables|Default|SetNextLoc "113959.632153,9298.951025,1800.000000")
                  (Timeline|Timeline PlayFromStart))
                (:7
                  (Variables|Default|SetNextLoc "121008.619321,1507.367848,1800.000000")
                  (Timeline|Timeline PlayFromStart))
                (:8
                  (Variables|Default|SetNextLoc "130440.559485,-4019.998881,1800.000000")
                  (Timeline|Timeline PlayFromStart))
                (:9
                  (Variables|Default|SetNextLoc "137983.762019,10522.768565,1800.000000")
                  (Timeline|Timeline PlayFromStart))
                (:10
                  (Variables|Default|SetNextLoc "149809.559759,2839.574109,1800.000000")
                  (Timeline|Timeline PlayFromStart)))))))
      (else
        (Variables|Default|SetbIsAnimFinished false)
        (Variables|Default|SetRot (Transformation|GetWorldRotation (Variables|Default|GetTowerTop)))
        (Variables|Default|SetLoc (Transformation|GetActorLocation))
        (Default|CallWarning)
        (bind (_direction_2 _a _rotatea_2) (Timeline|TimelineCancel PlayFromStart)
          (:Update
            (Transformation|SetActorLocation (Math|Vector|MakeVector (Math|Float|Lerp (.X (Math|Vector|BreakVector (Variables|Default|GetLoc))) (+ (.X (Math|Vector|BreakVector (Variables|Default|GetLoc))) 1e+02) _a) (Math|Float|Lerp (.Y (Math|Vector|BreakVector (Variables|Default|GetLoc))) (+ (.Y (Math|Vector|BreakVector (Variables|Default|GetLoc))) 1e+02) _a) (.Z (Math|Vector|BreakVector (Variables|Default|GetLoc)))) false false)
            (Transformation|SetWorldRotation (Variables|Default|GetTowerTop) (Math|Rotator|MakeRotator 0.0 0.0 (Math|Float|Lerp (.roll (Variables|Default|GetRot)) (+ (.roll (Variables|Default|GetRot)) 3.6e+02) _rotatea_2)) false false))
          (:Finished
            (Variables|Default|SetbIsAnimFinished true)))))
    (elif (> _standinglevel_2 1)
      (Math|Integer|DecrementInt _standinglevel
        (:%20%20
          (Variables|Default|SetChangedRotValue -1e+01)
          (goto _label)))
      (elif (== _standinglevel_2 1)
        (goto _label)))))

(event Custom|BackCustom
  (if (== (Variables|Default|GetStandingLevel) 0)
    _))

(event EventBeginPlay
  (bind _asbp_instance (Utilities|Casting|CastToBP_Instance (Game|GetGameInstance)))
  (Variables|Default|SetAs%20BP%20Instance _asbp_instance)
  (EventDispatchers|BindEventtoBack (delegate Custom|BackCustom)))

(fn ConstructionScript)