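; Laser curtain skill actor that stays hidden until SkillUse, then sweeps back and forth as a damaging beam.
; Four chained timelines lerp the actor from Loc1 through Loc2 to Loc3 and back, with short pauses between legs.
; Box overlaps deal fixed crit damage through BPI_Enemy, with a hit list limiting it to once per direction.
; The construction script offsets both end meshes by Distance and sizes the beam and box to span them.
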(event OnComponentBeginOverlap(Box)
  (params (OverlappedComponent :type Primitive%20Component%20Object%20Reference) (OtherActor :type Actor%20Object%20Reference) (OtherComp :type Primitive%20Component%20Object%20Reference) (OtherBodyIndex :type Integer) (bFromSweep :type Boolean) (SweepResult :type Hit%20Result%20Structure%20%28by%20ref%29))
  ;[0.15 0.15 0.15 0.5] Overlap
  (if (and (Utilities|DoesObjectImplementInterface OtherActor "/Game/_Game/BP/Frameworks/BPI_Enemy.BPI_Enemy_C") (not (Utilities|Array|ContainsItem (Variables|Default|GetHitEnemies1) OtherActor)))
    (Utilities|IsValid OtherActor
      (:Is%20Valid
        (Utilities|Array|Add (Variables|Default|GetHitEnemies1) OtherActor)
        (Game|SpawnActorfromClass "/Game/_Game/BP/BP_DamageText.BP_DamageText_C" (Math|Transform|MakeTransform (+ (Transformation|GetActorLocation OtherActor) "0.000000,0.000000,120.000000") "0, 0, 0" "1.000000,1.000000,1.000000") "Undefined" "MultiplyWithRoot" 0 45.0 true "" 0)
        (bind (_currenthealth _maxhealth) (Class|BPIEnemy|GetEnemyHealth(Message) OtherActor))
        (Class|BPIEnemy|SetHealth(Message) OtherActor (- _currenthealth 45.0) _maxhealth 0.0)
        (bind _currenthealth_2 (Class|BPIEnemy|GetEnemyHealth(Message) OtherActor))
        (Class|BPIEnemy|EnemyDamageTaken(Message) OtherActor)
        (if (<= _currenthealth_2 0.0)
          (Class|BPIEnemy|EnemyKilled(Message) OtherActor))))))

(event Custom|SkillUse
  (Rendering|SetVisibility (Variables|Default|GetP_Beam_02_Big) true false)
  (Audio|PlaySound2D "/Game/_Game/Sound/SFX/LaserCurtainSound.LaserCurtainSound" 1.0 1.0 0.0 0 0)
  (bind _a (Timeline|Timeline PlayFromStart)
    (:Update
      (Transformation|SetActorLocation (Math|Vector|Lerp(Vector) (Variables|Default|GetLoc1) (Variables|Default|GetLoc2) _a) false false))
    (:Finished
      (Utilities|FlowControl|Delay 0.25)
      (bind _a_2 (Timeline|Timeline_0 PlayFromStart)
        (:Update
          (Transformation|SetActorLocation (Math|Vector|Lerp(Vector) (Variables|Default|GetLoc2) (Variables|Default|GetLoc3) _a_2) false false))
        (:Finished
          (Utilities|FlowControl|Delay 0.25)
          (Utilities|Array|Clear (Variables|Default|GetHitEnemies1))
          (bind _a_3 (Timeline|Timeline_1 PlayFromStart)
            (:Update
              (Transformation|SetActorLocation (Math|Vector|Lerp(Vector) (Variables|Default|GetLoc3) (Variables|Default|GetLoc2) _a_3) false false))
            (:Finished
              (Utilities|FlowControl|Delay 0.25)
              (bind _a_4 (Timeline|Timeline_2 PlayFromStart)
                (:Update
                  (Transformation|SetActorLocation (Math|Vector|Lerp(Vector) (Variables|Default|GetLoc2) (Variables|Default|GetLoc1) _a_4) false false))
                (:Finished
                  (Rendering|SetVisibility (Variables|Default|GetP_Beam_02_Big) false false)
                  (Utilities|Array|Clear (Variables|Default|GetHitEnemies1)))))))))))

(event EventBeginPlay
  (Rendering|SetVisibility (Variables|Default|GetP_Beam_02_Big) false false))

(event EventTick
  (params (DeltaSeconds :type Float%20%28single-precision%29))
  (Transformation|AddLocalRotation (Variables|Default|GetStaticMesh2) (Math|Rotator|MakeRotator 0.0 0.0 (* (Utilities|Time|GetWorldDeltaSeconds) 7e+01)) false false))

(fn ConstructionScript
  (bind _sm1 (Variables|Default|GetSM1))
  (bind _p_beam_02_big (Variables|Default|GetP_Beam_02_Big))
  (bind _sm2 (Variables|Default|GetSM2))
  (bind _sm1_2 (Variables|Default|GetSM1))
  (bind _sm2_2 (Variables|Default|GetSM2))
  (bind _returnvalue (Transformation|GetWorldLocation _sm2_2))
  (bind _returnvalue_2 (Transformation|GetWorldLocation _sm1_2))
  (bind _relativelocation (Variables|/Script/Engine.SceneComponent|GetRelativeLocation _sm2))
  (bind _relativelocation_2 (Variables|/Script/Engine.SceneComponent|GetRelativeLocation _sm1))
  (bind _returnvalue_3 (Math|Vector|Distance(Vector) _returnvalue_2 _returnvalue))
  (Transformation|SetRelativeLocation _sm1 (Math|Vector|MakeVector (+ (.x _relativelocation_2) (* (Variables|Default|GetDistance) -1.0)) (.y _relativelocation_2) (.z _relativelocation_2)) false false)
  (Transformation|SetRelativeLocation _sm2 (Math|Vector|MakeVector (+ (.x _relativelocation) (Variables|Default|GetDistance)) (.y _relativelocation) (.z _relativelocation)) false false)
  (Transformation|SetWorldScale3D _p_beam_02_big (Math|Vector|MakeVector (/ _returnvalue_3 (/ (.x (Transformation|GetWorldScale _p_beam_02_big)) 0.002)) 2e+01 1e+01))
  (Components|Box|SetBoxExtent (Variables|Default|GetBox) (Math|Vector|MakeVector (/ _returnvalue_3 (/ (.x (Transformation|GetWorldScale (Variables|Default|GetBox))) 0.45)) 93.854885 1120.907528) true))