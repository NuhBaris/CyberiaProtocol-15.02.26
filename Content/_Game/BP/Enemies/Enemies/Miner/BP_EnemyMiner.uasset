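; Miner enemy that periodically overheats random towers in the level and handles its own death.
; After a delay it draws up to a set count of eligible towers, messages random picks and fires Niagara effects at them, repeating only if any qualified.
; Random indices are re-rolled at each use, so checked and affected towers can differ.
; A looping timer polls health; death pays the killing tower, notifies the spawner and destroys the actor.
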(event Custom|Check
  (if (<= (.CurrentHealth (Utilities|Struct|BreakStructure_Enemies (Variables|Default|GetEnemyData))) 0.0)
    (Rendering|SetVisibility (Variables|Default|GetW_HealthBar) false false)
    (if (not (Variables|Default|GetIsEnemyTakeDamage))
      (Utilities|FlowControl|DoOnce false
        (:Completed
          (Class|BPITowers|EnemyDied(Message) (stale EventEnemyKilled CausedTower) (.DropMoney (Utilities|Struct|BreakStructure_Enemies (Variables|Default|GetEnemyData))))
          (Niagara|SpawnSystematLocation "/Game/_Game/Niagara/NS_EnemyDie.NS_EnemyDie" (.location (Transformation|GetActorTransform)))
          (bind _outactors (Actor|GetAllActorsOfClass "/Game/_Game/BP/Enemies/BP_EnemySpawner.BP_EnemySpawner_C"))
          (Class|BPIGeneral|EnemyDiedGeneral(Message) (Utilities|Array|Get(acopy) _outactors))
          (Actor|DestroyActor))))))

(event EventBeginPlay
  (bind _overheatabletowerstemp (Variables|Default|GetOverheatableTowersTemp))
  (bind _returnvalue (Utilities|Array|Length _overheatabletowerstemp))
  (bind _returnvalue_2 (- _returnvalue 1))
  (bind _returnvalue_3 (Math|Random|RandomIntegerinRange 0 _returnvalue_2))
  (bind _output (Utilities|Array|Get(acopy) _overheatabletowerstemp _returnvalue_3))
  (|CallParentFunction)
  (Variables|Default|SetOverheatTowerCountTemp (Variables|Default|GetOverheatTowerCount))
  (Utilities|Time|SetTimerbyEvent (delegate Custom|Check) 0.05 true)
  (Utilities|FlowControl|Delay (Variables|Default|GetOverheatSkillTime) :!label _label)
  (Utilities|IsValid self
    (:Is%20Valid
      (bind _outactors (Actor|GetAllActorsOfClass "/Game/_Game/BP/Towers/Towers/BP_TowerBase.BP_TowerBase_C"))
      (bind _output_get (Variables|Default|SetCurrentTowers _outactors))
      (for _array_element _outactors
        (if (and (not (Variables|/Game/_Game/BP/Towers/Towers/BP_TowerBase.BP_TowerBase_C|GetbIsOverheated (Utilities|Array|Get(acopy) _output_get (Math|Random|RandomIntegerinRange 0 (- (Utilities|Array|Length _output_get) 1))))) (Variables|/Game/_Game/BP/Towers/Towers/BP_TowerBase.BP_TowerBase_C|GetbCanOverheat (Utilities|Array|Get(acopy) _output_get (Math|Random|RandomIntegerinRange 0 (- (Utilities|Array|Length _output_get) 1)))))
          (Utilities|FlowControl|DoN (Variables|Default|GetOverheatTowerCount)
            (:Exit
              (Utilities|Array|Add (Variables|Default|GetOverheatableTowers) (Utilities|Array|Get(acopy) _output_get (Math|Random|RandomIntegerinRange 0 (- (Utilities|Array|Length _output_get) 1))))
              (Utilities|Array|Add (Variables|Default|GetOverheatableTowersTemp) (Utilities|Array|Get(acopy) _output_get (Math|Random|RandomIntegerinRange 0 (- (Utilities|Array|Length _output_get) 1))))
              (Utilities|Array|RemoveItem (Variables|Default|GetCurrentTowers) (Utilities|Array|Get(acopy) _output_get (Math|Random|RandomIntegerinRange 0 (- (Utilities|Array|Length _output_get) 1))))))
          (else
            (Utilities|Array|RemoveItem (Variables|Default|GetCurrentTowers) (Utilities|Array|Get(acopy) _output_get (Math|Random|RandomIntegerinRange 0 (- (Utilities|Array|Length _output_get) 1)))))))
      (if (!= (Utilities|Array|Length (Variables|Default|GetOverheatableTowers)) 0)
        (for _array_element_2 (Variables|Default|GetOverheatableTowers)
          (Class|BPITowers|OverheatSelectedTower(Message) _output)
          (bind _returnvalue_4 (Niagara|SpawnSystematLocation "/Game/_Game/Niagara/NS_Miner.NS_Miner" (Transformation|GetActorLocation)))
          (Variables|Default|SetTowerLoc (Transformation|GetActorLocation _output))
          (Niagara|SetNiagaraVariable(Vector3) _returnvalue_4 "TargetPosition" (Math|Vector|MakeVector (.x (Variables|Default|GetTowerLoc)) (.y (Variables|Default|GetTowerLoc)) (+ (.z (Variables|Default|GetTowerLoc)) 1.5e+02)))
          (Niagara|SetNiagaraVariable(LinearColor) _returnvalue_4 "Color" (Utilities|Struct|MakeLinearColor 1.0 0.654823 0.0 1.0))
          (Niagara|SetNiagaraVariable(Float) _returnvalue_4 "BulletSize" 4e+01))
        (Utilities|Array|Clear (Variables|Default|GetOverheatableTowersTemp))
        (Utilities|Array|Clear (Variables|Default|GetOverheatableTowers))
        (Utilities|FlowControl|Sequence
          (:then_0
            (goto _label))
          (:then_1
            (Utilities|FlowControl|DoN (Variables|Default|GetOverheatTowerCount)) ; enters at Reset
          ))))))

(event EventEnemyKilled
  (params (CausedTower :type BP%20Tower%20Base%20Object%20Reference))
  (if (not (Variables|Default|GetIsEnemyTakeDamage))
    (Utilities|FlowControl|DoOnce false
      (:Completed
        (Class|BPITowers|EnemyDied(Message) CausedTower (.DropMoney (Utilities|Struct|BreakStructure_Enemies (Variables|Default|GetEnemyData))))
        (Niagara|SpawnSystematLocation "/Game/_Game/Niagara/NS_EnemyDie.NS_EnemyDie" (.location (Transformation|GetActorTransform)))
        (bind _outactors (Actor|GetAllActorsOfClass "/Game/_Game/BP/Enemies/BP_EnemySpawner.BP_EnemySpawner_C"))
        (Class|BPIGeneral|EnemyDiedGeneral(Message) (Utilities|Array|Get(acopy) _outactors))
        (Actor|DestroyActor)))))

(fn ConstructionScript
  (|CallParentFunction))