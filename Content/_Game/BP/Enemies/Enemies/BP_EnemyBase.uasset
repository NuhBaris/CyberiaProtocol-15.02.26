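; Base tower-defense enemy that follows the BP_EnemyPath spline on a looping timer, with scale-in on spawn and a camera-facing health bar.
; At path end it damages the base, messages the player, shrinks away, notifies the spawner and destroys itself.
; EnemyEffect applies fire damage ticks or timed slow and freeze by rewriting the EnemyData struct.
; Interface events and getters expose health, speed and path progress, while a dynamic material drives hit flashes.
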(event Custom|CustomEvent
  (bind _staticmesh (Variables|Default|GetStaticMesh))
  (bind _staticmeshscale (Variables|Default|GetStaticMeshScale))
  (bind _enemypath (Variables|Default|GetEnemyPath))
  (bind _returnvalue (Transformation|GetWorldLocation _staticmesh))
  (bind _spline_enemypath (Variables|/Game/_Game/BP/Enemies/BP_EnemyPath.BP_EnemyPath_C|GetSpline_EnemyPath _enemypath))
  ;[0.15 0.15 0.15 0.5] Beginplay
  (bind _output_get (Variables|Default|SetDistanceOnSpline (Math|Float|Clamp(Float) (+ (Variables|Default|GetDistanceOnSpline) (.Speed (Utilities|Struct|BreakStructure_Enemies (Variables|Default|GetEnemyData)))) 0.0 (Spline|GetSplineLength _spline_enemypath))))
  (Transformation|SetActorTransform (Math|Transform|MakeTransform (Spline|GetLocationatDistanceAlongSpline _spline_enemypath _output_get "World") (Spline|GetRotationatDistanceAlongSpline _spline_enemypath _output_get "World") "1.000000,1.000000,1.000000"))
  (Utilities|FlowControl|Sequence
    (:then_0
      (if (>= (Variables|Default|GetDistanceOnSpline) (Spline|GetSplineLength (Variables|/Game/_Game/BP/Enemies/BP_EnemyPath.BP_EnemyPath_C|GetSpline_EnemyPath (Variables|Default|GetEnemyPath))))
        (Utilities|IsValid self
          (:Is%20Valid
            (Utilities|FlowControl|DoOnce false
              (:Completed
                (bind _outactors (Actor|GetAllActorsOfClass "/Game/_Game/BP/BP_Base.BP_Base_C"))
                (Default|DamageTaken (Utilities|Array|Get(acopy) _outactors))
                (Class|BPIGeneral|DamageTakenInterface(Message) (Game|GetPlayerCharacter 0) (.Damage (Utilities|Struct|BreakStructure_Enemies (Variables|Default|GetEnemyData))) 0.0 0.0)
                (Variables|Default|SetIsEnemyTakeDamage true)
                (Rendering|SetVisibility (Variables|Default|GetW_HealthBar) false false)
                (bind _a (Timeline|Timeline Play)
                  (:Update
                    (Transformation|SetWorldScale3D _staticmesh (Math|Vector|MakeVector (Math|Float|Lerp (.x _staticmeshscale) 0.0 _a) (Math|Float|Lerp (.y _staticmeshscale) 0.0 _a) (Math|Float|Lerp (.z _staticmeshscale) 0.0 _a)))
                    (Transformation|SetWorldLocation (Variables|Default|GetStaticMesh) (Math|Vector|MakeVector (Math|Float|Lerp (.x _returnvalue) (+ (.x _returnvalue) -3e+01) _a) (.y _returnvalue) (Math|Float|Lerp (.z _returnvalue) (+ (.z _returnvalue) 3e+01) _a)) false false))
                  (:Finished
                    (bind _outactors_2 (Actor|GetAllActorsOfClass "/Game/_Game/BP/Enemies/BP_EnemySpawner.BP_EnemySpawner_C"))
                    (Class|BPIGeneral|EnemyDiedGeneral(Message) (Utilities|Array|Get(acopy) _outactors_2))
                    (Actor|DestroyActor)))))))))
    (:then_1
      (Utilities|IsValid self
        (:Is%20Valid
          (Transformation|SetWorldRotation (Variables|Default|GetW_HealthBar) (Math|Rotator|FindLookatRotation (Transformation|GetWorldLocation (Variables|Default|GetW_HealthBar)) (Camera|GetCameraLocation (Game|GetPlayerCameraManager 0))) false false))))))

(event Custom|TakeFire
  ;[0.15 0.15 0.15 0.5] Effect
  (Utilities|IsValid self
    (:Is%20Valid
      (if (== (Variables|Default|GetFireLoopCount) 2)
        (Variables|Default|SetbFireLoop false)
        (else
          (Math|Integer|IncrementInt (Variables|Default|GetFireLoopCount)
            (:%20%20
              (Niagara|SpawnSystemAttached "/Game/_Game/Niagara/NS_FireHit.NS_FireHit" (Variables|Default|GetStaticMesh) "None" "0, 0, 0" "0, 0, 0" "SnapToTarget" true)
              (Game|SpawnActorfromClass "/Game/_Game/BP/BP_DamageText.BP_DamageText_C" (Math|Transform|MakeTransform (+ (Transformation|GetActorLocation) "0.000000,0.000000,120.000000") "0, 0, 0" "1.000000,1.000000,1.000000") "Undefined" "MultiplyWithRoot" 0 (stale EventEnemyEffect FireDamage) false 0)
              (Utilities|IsValid (stale EventEnemyEffect Tower)
                (:Is%20Valid
                  (Class|BPITowers|EnemyTakeFireDamage(Message) (stale EventEnemyEffect Tower) self 0.0))
                (:Is%20Not%20Valid
                  _))
              (Variables|Default|SetEnemyData (Utilities|Struct|MakeStructure_Enemies (.IsAlive (Utilities|Struct|BreakStructure_Enemies (Variables|Default|GetEnemyData))) (- (.CurrentHealth (Utilities|Struct|BreakStructure_Enemies (Variables|Default|GetEnemyData))) (stale EventEnemyEffect FireDamage)) (.MaxHealth (Utilities|Struct|BreakStructure_Enemies (Variables|Default|GetEnemyData))) (.Speed (Utilities|Struct|BreakStructure_Enemies (Variables|Default|GetEnemyData))) (.Damage (Utilities|Struct|BreakStructure_Enemies (Variables|Default|GetEnemyData))) (.DropMoney (Utilities|Struct|BreakStructure_Enemies (Variables|Default|GetEnemyData))))))))))))

(event EventBeginPlay
  (bind _enemydata (Variables|Default|GetEnemyData))
  (bind (_isalive _currenthealth _maxhealth) (Utilities|Struct|BreakStructure_Enemies _enemydata))
  ;[0.15 0.15 0.15 0.5] Beginplay
  (bind _returnvalue (Rendering|Material|CreateDynamicMaterialInstance (Variables|Default|GetStaticMesh) 0 0 "None" :!class /Script/Engine.PrimitiveComponent))
  (Variables|Default|SetDynamicMat _returnvalue)
  (Variables|Default|SetStaticMeshScale (Transformation|GetWorldScale (Variables|Default|GetStaticMesh)))
  (Utilities|Time|SetTimerbyEvent (delegate Custom|CustomEvent) 0.02 true)
  (bind _outactors (Actor|GetAllActorsOfClass "/Game/_Game/BP/Enemies/BP_EnemyPath.BP_EnemyPath_C"))
  (Variables|Default|SetEnemyPath (Utilities|Array|Get(acopy) _outactors))
  (Transformation|SetRelativeLocation (Variables|Default|GetW_HealthBar) (Math|Vector|MakeVector 0.0 0.0 (+ (.z (.BoxExtent (Collision|GetComponentBounds (Variables|Default|GetStaticMesh)))) 2e+02)) false false)
  (Class|BPIEnemy|SetHealthWidget(Message) (UserInterface|GetUserWidgetObject (Variables|Default|GetW_HealthBar)) _currenthealth _maxhealth)
  (bind _a (Timeline|Timeline_0 Play)
    (:Update
      (Transformation|SetWorldScale3D (Variables|Default|GetStaticMesh) (Math|Vector|MakeVector (Math|Float|Lerp 0.0 (.x (Variables|Default|GetStaticMeshScale)) _a) (Math|Float|Lerp 0.0 (.y (Variables|Default|GetStaticMeshScale)) _a) (Math|Float|Lerp 0.0 (.z (Variables|Default|GetStaticMeshScale)) _a))))
    (:Finished
      (Rendering|SetVisibility (Variables|Default|GetW_HealthBar) true false))))

(event EventEnemyDamageTaken
  ;[0.15 0.15 0.15 0.5] Materyal
  (bind _a (Timeline|Timeline_1 PlayFromStart)
    (:Update
      (Rendering|Material|SetScalarParameterValue (Variables|Default|GetDynamicMat) "HitFlash" _a :!class /Script/Engine.MaterialInstanceDynamic))))

(event EventEnemyEffect
  (params (EffectType :type String) (Tower :type BP%20Tower%20Base%20Object%20Reference) (FireDamage :type Float%20%28double-precision%29) (FireDuration :type Float%20%28double-precision%29) (SlowDuration :type Float%20%28double-precision%29) (SlowAmount :type Float%20%28double-precision%29))
  ;[0.15 0.15 0.15 0.5] Effect
  (switch string EffectType
    (:Fire
      (Variables|Default|SetbFireLoop true)
      (Variables|Default|SetFireLoopCount 0)
      (Utilities|Time|SetTimerbyEvent (delegate Custom|TakeFire) FireDuration (Variables|Default|GetbFireLoop)))
    (:Slow
      (if (and (Variables|Default|GetbIsNormalSpeed) (not (Variables|Default|GetbIsFreeze)))
        (Variables|Default|SetLastSpeed (.Speed (Utilities|Struct|BreakStructure_Enemies (Variables|Default|GetEnemyData))))
        (Variables|Default|SetbIsNormalSpeed false)
        (Variables|Default|SetEnemyData (Utilities|Struct|MakeStructure_Enemies (.IsAlive (Utilities|Struct|BreakStructure_Enemies (Variables|Default|GetEnemyData))) (.CurrentHealth (Utilities|Struct|BreakStructure_Enemies (Variables|Default|GetEnemyData))) (.MaxHealth (Utilities|Struct|BreakStructure_Enemies (Variables|Default|GetEnemyData))) (- (.Speed (Utilities|Struct|BreakStructure_Enemies (Variables|Default|GetEnemyData))) (/ (* (.Speed (Utilities|Struct|BreakStructure_Enemies (Variables|Default|GetEnemyData))) SlowAmount) 1e+02)) (.Damage (Utilities|Struct|BreakStructure_Enemies (Variables|Default|GetEnemyData))) (.DropMoney (Utilities|Struct|BreakStructure_Enemies (Variables|Default|GetEnemyData)))))
        (Niagara|SpawnSystemAttached "/Game/_Game/Niagara/NS_SlowHit.NS_SlowHit" (Variables|Default|GetStaticMesh) "None" "0, 0, 0" "0, 0, 0" "SnapToTarget" true)
        (Utilities|FlowControl|Delay 2.0)
        (Variables|Default|SetEnemyData (Utilities|Struct|MakeStructure_Enemies (.IsAlive (Utilities|Struct|BreakStructure_Enemies (Variables|Default|GetEnemyData))) (.CurrentHealth (Utilities|Struct|BreakStructure_Enemies (Variables|Default|GetEnemyData))) (.MaxHealth (Utilities|Struct|BreakStructure_Enemies (Variables|Default|GetEnemyData))) (Variables|Default|GetLastSpeed) (.Damage (Utilities|Struct|BreakStructure_Enemies (Variables|Default|GetEnemyData))) (.DropMoney (Utilities|Struct|BreakStructure_Enemies (Variables|Default|GetEnemyData)))))
        (Variables|Default|SetbIsNormalSpeed true)))
    (:Freeze
      (if (and (Variables|Default|GetbIsNormalSpeed) (not (Variables|Default|GetbIsFreeze)))
        (Variables|Default|SetLastSpeed (.Speed (Utilities|Struct|BreakStructure_Enemies (Variables|Default|GetEnemyData))))
        (Variables|Default|SetbIsNormalSpeed false)
        (Variables|Default|SetbIsFreeze true)
        (Variables|Default|SetEnemyData (Utilities|Struct|MakeStructure_Enemies (.IsAlive (Utilities|Struct|BreakStructure_Enemies (Variables|Default|GetEnemyData))) (.CurrentHealth (Utilities|Struct|BreakStructure_Enemies (Variables|Default|GetEnemyData))) (.MaxHealth (Utilities|Struct|BreakStructure_Enemies (Variables|Default|GetEnemyData))) 0.0 (.Damage (Utilities|Struct|BreakStructure_Enemies (Variables|Default|GetEnemyData))) (.DropMoney (Utilities|Struct|BreakStructure_Enemies (Variables|Default|GetEnemyData)))))
        (Niagara|SpawnSystemAttached "/Game/_Game/Niagara/NS_SlowHit.NS_SlowHit" (Variables|Default|GetStaticMesh) "None" "0, 0, 0" "0, 0, 0" "SnapToTarget" true)
        (Utilities|FlowControl|Delay 3.0)
        (Variables|Default|SetEnemyData (Utilities|Struct|MakeStructure_Enemies (.IsAlive (Utilities|Struct|BreakStructure_Enemies (Variables|Default|GetEnemyData))) (.CurrentHealth (Utilities|Struct|BreakStructure_Enemies (Variables|Default|GetEnemyData))) (.MaxHealth (Utilities|Struct|BreakStructure_Enemies (Variables|Default|GetEnemyData))) (Variables|Default|GetLastSpeed) (.Damage (Utilities|Struct|BreakStructure_Enemies (Variables|Default|GetEnemyData))) (.DropMoney (Utilities|Struct|BreakStructure_Enemies (Variables|Default|GetEnemyData)))))
        (Variables|Default|SetbIsNormalSpeed true)
        (Variables|Default|SetbIsFreeze false)))))

(event EventSetHealth
  (params (CurrentHealth :type Float%20%28double-precision%29) (MaxHealth :type Float%20%28double-precision%29))
  ;[0.15 0.15 0.15 0.5] Interface
  (Variables|Default|SetEnemyData (Utilities|Struct|MakeStructure_Enemies (.IsAlive (Utilities|Struct|BreakStructure_Enemies (Variables|Default|GetEnemyData))) CurrentHealth (.MaxHealth (Utilities|Struct|BreakStructure_Enemies (Variables|Default|GetEnemyData))) (.Speed (Utilities|Struct|BreakStructure_Enemies (Variables|Default|GetEnemyData))) (.Damage (Utilities|Struct|BreakStructure_Enemies (Variables|Default|GetEnemyData))) (.DropMoney (Utilities|Struct|BreakStructure_Enemies (Variables|Default|GetEnemyData)))))
  (Class|BPIEnemy|SetHealthWidget(Message) (UserInterface|GetUserWidgetObject (Variables|Default|GetW_HealthBar)) CurrentHealth MaxHealth))

(fn ConstructionScript)

(fn GetEnemyHealth
  (bind _enemydata (Variables|Default|GetEnemyData))
  (bind (_isalive _currenthealth _maxhealth) (Utilities|Struct|BreakStructure_Enemies _enemydata))
  (return _currenthealth _maxhealth))

(fn GetEnemyMesh
  (return (Variables|Default|GetStaticMesh)))

(fn GetEnemySpeed
  (return (.Speed (Utilities|Struct|BreakStructure_Enemies (Variables|Default|GetEnemyData)))))

(fn GetLength
  (return (Variables|Default|GetDistanceOnSpline) (Spline|GetSplineLength (Variables|/Game/_Game/BP/Enemies/BP_EnemyPath.BP_EnemyPath_C|GetSpline_EnemyPath (Variables|Default|GetEnemyPath)))))