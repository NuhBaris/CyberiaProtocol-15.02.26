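; Enemy entity Blueprint that handles an enemy's death.
; A looping timer polls current health and hides the health bar at zero, while an EnemyKilled event enters the same death path directly.
; When IsEnemyTakeDamage is false, that path runs once: it reports drop money to the causing tower, spawns a Niagara death effect, notifies the first BP_EnemySpawner found and destroys the actor.
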(event Custom|Check
  (if (<= (.CurrentHealth (Utilities|Struct|BreakStructure_Enemies (Variables|Default|GetEnemyData))) 0.0)
    (Rendering|SetVisibility (Variables|Default|GetW_HealthBar) false false)
    (if (not (Variables|Default|GetIsEnemyTakeDamage))
      (Utilities|FlowControl|DoOnce false
        (:Completed
          (Class|BPITowers|EnemyDied(Message) (stale EventEnemyKilled CausedTower) (.DropMoney (Utilities|Struct|BreakStructure_Enemies (Variables|Default|GetEnemyData))))
          (Niagara|SpawnSystematLocation "/Game/_Game/Niagara/NS_EnemyDie.NS_EnemyDie" (.location (Transformation|GetActorTransform)))
          (bind _outactors (Actor|GetAllActorsOfClass "/Game/_Game/BP/Enemies/BP_EnemySpawner.BP_EnemySpawner_C"))
          (Class|BPIGeneral|EnemyDiedGeneral(Message) (Utilities|Array|Get(acopy) _outactors))
          (Actor|DestroyActor))))))

(event EventBeginPlay
  (|CallParentFunction)
  (Utilities|Time|SetTimerbyEvent (delegate Custom|Check) 0.05 true))

(event EventEnemyKilled
  (params (CausedTower :type BP%20Tower%20Base%20Object%20Reference))
  (if (not (Variables|Default|GetIsEnemyTakeDamage))
    (Utilities|FlowControl|DoOnce false
      (:Completed
        (Class|BPITowers|EnemyDied(Message) CausedTower (.DropMoney (Utilities|Struct|BreakStructure_Enemies (Variables|Default|GetEnemyData))))
        (Niagara|SpawnSystematLocation "/Game/_Game/Niagara/NS_EnemyDie.NS_EnemyDie" (.location (Transformation|GetActorTransform)))
        (bind _outactors (Actor|GetAllActorsOfClass "/Game/_Game/BP/Enemies/BP_EnemySpawner.BP_EnemySpawner_C"))
        (Class|BPIGeneral|EnemyDiedGeneral(Message) (Utilities|Array|Get(acopy) _outactors))
        (Actor|DestroyActor)))))

(fn ConstructionScript
  (|CallParentFunction))