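; Trojan enemy for the tower defense game that, on death, releases a group of random enemies from the spawner's available list.
; A looping timer polls health and shares a one-shot death path with EnemyKilled, gated on IsEnemyTakeDamage being false.
; That path sends the money drop to the killing tower, plays a Niagara effect and notifies the spawner.
; Spawned enemies inherit the Trojan's spline distance, with per-index offsets spreading the first five apart.
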(event Custom|Check
  (if (<= (.CurrentHealth (Utilities|Struct|BreakStructure_Enemies (Variables|Default|GetEnemyData))) 0.0)
    (Rendering|SetVisibility (Variables|Default|GetW_HealthBar) false false)
    (if (not (Variables|Default|GetIsEnemyTakeDamage))
      (Utilities|FlowControl|DoOnce false
        (:Completed
          (Class|BPITowers|EnemyDied(Message) (stale EventEnemyKilled CausedTower) (.DropMoney (Utilities|Struct|BreakStructure_Enemies (Variables|Default|GetEnemyData))))
          (Niagara|SpawnSystematLocation "/Game/_Game/Niagara/NS_EnemyDie.NS_EnemyDie" (.location (Transformation|GetActorTransform)))
          (bind _outactors (Actor|GetAllActorsOfClass "/Game/_Game/BP/Enemies/BP_EnemySpawner.BP_EnemySpawner_C"))
          (Class|BPIGeneral|EnemyDiedGeneral(Message) (Utilities|Array|Get(acopy) _outactors))
          (bind _enemylist (Class|BPIGeneral|GetAvailableEnemyList(Message) (Utilities|Array|Get(acopy) _outactors)))
          (Variables|Default|SetLastSplineDistance (Variables|Default|GetDistanceOnSpline))
          (for _index (range 1 (Variables|Default|GetSpawnEnemyCount))
            (bind _returnvalue (Game|SpawnActorfromClass (.EnemyClass (Utilities|Struct|BreakStructure_EnemyData (Utilities|Array|Get(acopy) _enemylist (Math|Random|RandomInteger (Utilities|Array|Length _enemylist))))) (Math|Transform|MakeTransform (Transformation|GetActorLocation) "0, 0, 0" "1.000000,1.000000,1.000000") "Undefined" "MultiplyWithRoot" 0 false 0))
            (Variables|/Game/_Game/BP/Enemies/Enemies/BP_EnemyBase.BP_EnemyBase_C|SetDistanceOnSpline _returnvalue (Variables|Default|GetLastSplineDistance))
            (switch int _index
              (:1
                (Variables|/Game/_Game/BP/Enemies/Enemies/BP_EnemyBase.BP_EnemyBase_C|SetSplineDistanceX _returnvalue 0.0)
                (Variables|/Game/_Game/BP/Enemies/Enemies/BP_EnemyBase.BP_EnemyBase_C|SetSplineDistanceY _returnvalue 0.0))
              (:2
                (Variables|/Game/_Game/BP/Enemies/Enemies/BP_EnemyBase.BP_EnemyBase_C|SetSplineDistanceX _returnvalue 1e+02)
                (Variables|/Game/_Game/BP/Enemies/Enemies/BP_EnemyBase.BP_EnemyBase_C|SetSplineDistanceY _returnvalue 0.0))
              (:3
                (Variables|/Game/_Game/BP/Enemies/Enemies/BP_EnemyBase.BP_EnemyBase_C|SetSplineDistanceX _returnvalue -1e+02)
                (Variables|/Game/_Game/BP/Enemies/Enemies/BP_EnemyBase.BP_EnemyBase_C|SetSplineDistanceY _returnvalue 0.0))
              (:4
                (Variables|/Game/_Game/BP/Enemies/Enemies/BP_EnemyBase.BP_EnemyBase_C|SetSplineDistanceX _returnvalue 1e+02)
                (Variables|/Game/_Game/BP/Enemies/Enemies/BP_EnemyBase.BP_EnemyBase_C|SetSplineDistanceY _returnvalue 1e+02))
              (:5
                (Variables|/Game/_Game/BP/Enemies/Enemies/BP_EnemyBase.BP_EnemyBase_C|SetSplineDistanceX _returnvalue -1e+02)
                (Variables|/Game/_Game/BP/Enemies/Enemies/BP_EnemyBase.BP_EnemyBase_C|SetSplineDistanceY _returnvalue 1e+02))))
          (Actor|DestroyActor))))))

(event EventBeginPlay
  (|CallParentFunction)
  (Utilities|Time|SetTimerbyEvent (delegate Custom|Check) 0.05 true))

(event EventEnemyKilled
  (params (CausedTower :type BP%20Tower%20Base%20Object%20Reference))
  (if (not (Variables|Default|GetIsEnemyTakeDamage))
    (Utilities|FlowControl|DoOnce false
      (:Completed
        (Class|BPITowers|EnemyDied(Message) CausedTower (.DropMoney (Utilities|Struct|BreakStructure_Enemies (Variables|Default|GetEnemyData))))
        (Niagara|SpawnSystematLocation "/Game/_Game/Niagara/NS_EnemyDie.NS_EnemyDie" (.location (Transformation|GetActorTransform)))
        (bind _outactors (Actor|GetAllActorsOfClass "/Game/_Game/BP/Enemies/BP_EnemySpawner.BP_EnemySpawner_C"))
        (Class|BPIGeneral|EnemyDiedGeneral(Message) (Utilities|Array|Get(acopy) _outactors))
        (bind _enemylist (Class|BPIGeneral|GetAvailableEnemyList(Message) (Utilities|Array|Get(acopy) _outactors)))
        (Variables|Default|SetLastSplineDistance (Variables|Default|GetDistanceOnSpline))
        (for _index (range 1 (Variables|Default|GetSpawnEnemyCount))
          (bind _returnvalue (Game|SpawnActorfromClass (.EnemyClass (Utilities|Struct|BreakStructure_EnemyData (Utilities|Array|Get(acopy) _enemylist (Math|Random|RandomInteger (Utilities|Array|Length _enemylist))))) (Math|Transform|MakeTransform (Transformation|GetActorLocation) "0, 0, 0" "1.000000,1.000000,1.000000") "Undefined" "MultiplyWithRoot" 0 false 0))
          (Variables|/Game/_Game/BP/Enemies/Enemies/BP_EnemyBase.BP_EnemyBase_C|SetDistanceOnSpline _returnvalue (Variables|Default|GetLastSplineDistance))
          (switch int _index
            (:1
              (Variables|/Game/_Game/BP/Enemies/Enemies/BP_EnemyBase.BP_EnemyBase_C|SetSplineDistanceX _returnvalue 0.0)
              (Variables|/Game/_Game/BP/Enemies/Enemies/BP_EnemyBase.BP_EnemyBase_C|SetSplineDistanceY _returnvalue 0.0))
            (:2
              (Variables|/Game/_Game/BP/Enemies/Enemies/BP_EnemyBase.BP_EnemyBase_C|SetSplineDistanceX _returnvalue 1e+02)
              (Variables|/Game/_Game/BP/Enemies/Enemies/BP_EnemyBase.BP_EnemyBase_C|SetSplineDistanceY _returnvalue 0.0))
            (:3
              (Variables|/Game/_Game/BP/Enemies/Enemies/BP_EnemyBase.BP_EnemyBase_C|SetSplineDistanceX _returnvalue -1e+02)
              (Variables|/Game/_Game/BP/Enemies/Enemies/BP_EnemyBase.BP_EnemyBase_C|SetSplineDistanceY _returnvalue 0.0))
            (:4
              (Variables|/Game/_Game/BP/Enemies/Enemies/BP_EnemyBase.BP_EnemyBase_C|SetSplineDistanceX _returnvalue 1e+02)
              (Variables|/Game/_Game/BP/Enemies/Enemies/BP_EnemyBase.BP_EnemyBase_C|SetSplineDistanceY _returnvalue 1e+02))
            (:5
              (Variables|/Game/_Game/BP/Enemies/Enemies/BP_EnemyBase.BP_EnemyBase_C|SetSplineDistanceX _returnvalue -1e+02)
              (Variables|/Game/_Game/BP/Enemies/Enemies/BP_EnemyBase.BP_EnemyBase_C|SetSplineDistanceY _returnvalue 1e+02))))
        (Actor|DestroyActor)))))

(fn ConstructionScript
  (|CallParentFunction))