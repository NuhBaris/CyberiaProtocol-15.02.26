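; Enemy wave spawner that advances rounds, builds each wave from a round-scaled budget and reports progress to the player's layout UI.
; Each wave rolls Normal, Swarm, Tank or Fast, biasing a weighted random pick by cost, speed and peak-round proximity.
; Picks fill a queue until the budget runs out, then spawn at the spawner with random delays.
; EnemyDiedGeneral unlocks the next round once at most one enemy remains and the queue is empty.
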(event Custom|GenerateQueue
  (while (> (Variables|Default|GetTempBudget) 0)
    (bind (_enemydata _isvalid) (CallFunction|PickEnemy (Math|Conversions|ToFloat(Integer) (Variables|Default|GetCurrentRound))))
    (if _isvalid
      (if (<= (.Cost (Utilities|Struct|BreakStructure_EnemyData _enemydata)) (Variables|Default|GetTempBudget))
        (Utilities|Array|Add (Variables|Default|GetSpawnQueue%20) (.EnemyClass (Utilities|Struct|BreakStructure_EnemyData _enemydata)))
        (Variables|Default|SetTempBudget (Math|Float|Truncate (- (Variables|Default|GetTempBudget) (.Cost (Utilities|Struct|BreakStructure_EnemyData _enemydata))))))
      (else
        (Variables|Default|SetTempBudget 0)))))

(event Custom|SpawnFromQueue
  (bind _spawnqueue_ (Variables|Default|GetSpawnQueue%20))
  (if (> (Utilities|Array|Length _spawnqueue_) 0)
    (Game|SpawnActorfromClass (Utilities|Array|Get(acopy) _spawnqueue_) (Math|Transform|MakeTransform (Transformation|GetActorLocation) "0, 0, 0" "1.000000,1.000000,1.000000") "Undefined" "MultiplyWithRoot" 0 0)
    (Utilities|Array|RemoveIndex _spawnqueue_)
    (Utilities|FlowControl|Delay (Math|Random|RandomFloatinRange 0.7 1.0))
    (CallFunction|SpawnfromQueue)))

(event Custom|SpawnWave
  (switch int (Math|Random|RandomIntegerinRange 0 3)
    (:0
      (Variables|Default|SetCurrentWaveType%20 "NewEnumerator0"))
    (:1
      (Variables|Default|SetCurrentWaveType%20 "NewEnumerator1"))
    (:2
      (Variables|Default|SetCurrentWaveType%20 "NewEnumerator2"))
    (:3
      (Variables|Default|SetCurrentWaveType%20 "NewEnumerator3")))
  (Development|PrintString (Utilities|String|EnumtoString (Variables|Default|GetCurrentWaveType%20)))
  (bind _bugdet (CallFunction|CalculateBudget (Math|Conversions|ToFloat(Integer) (Variables|Default|GetCurrentRound))))
  (bind _output_get (Variables|Default|SetCurrentBudget (Math|Float|Truncate _bugdet)))
  (Variables|Default|SetTempBudget _output_get)
  (Utilities|FlowControl|Delay 0.2)
  (CallFunction|GenerateQueue)
  (Utilities|FlowControl|Delay 0.1)
  (CallFunction|SpawnfromQueue))

(event EventBeginPlay
  (Utilities|FlowControl|Delay 0.2)
  (bind _wlayout (Class|BPIGeneral|GetWLayout(Message) (Game|Player|GetPlayerPawn 0)))
  (Default|NextRoundInterfaceF _wlayout (Variables|Default|GetCurrentRound) (Variables|Default|GetMaxRound)))

(event EventEnemyDiedGeneral
  (bind _outactors (Actor|GetAllActorsOfClass "/Game/_Game/BP/Enemies/Enemies/BP_EnemyBase.BP_EnemyBase_C"))
  (if (and (or (== (Utilities|Array|Length _outactors) 1) (== (Utilities|Array|Length _outactors) 0)) (== (Utilities|Array|Length (Variables|Default|GetSpawnQueue%20)) 0))
    (Variables|Default|SetbCanPassNextRaound true)
    (bind _wlayout (Class|BPIGeneral|GetWLayout(Message) (Game|Player|GetPlayerPawn 0)))
    (Class|BPIGeneral|RoundEnded(Message) _wlayout)))

(event EventNextWave
  (if (and (< (Variables|Default|GetCurrentRound) (Variables|Default|GetMaxRound)) (Variables|Default|GetbCanPassNextRaound))
    (Variables|Default|SetbCanPassNextRaound false)
    (Class|BPIGeneral|GetCurrentRound(Message) (Game|GetPlayerCharacter 0) (Variables|Default|GetCurrentRound))
    (Variables|Default|SetCurrentRound (+ (Variables|Default|GetCurrentRound) 1))
    (CallFunction|SpawnWave)
    (bind _wlayout (Class|BPIGeneral|GetWLayout(Message) (Game|Player|GetPlayerPawn 0)))
    (Default|NextRoundInterfaceF _wlayout (Variables|Default|GetCurrentRound) (Variables|Default|GetMaxRound))))

(fn ConstructionScript)

(fn CreateEnemy
  (bind _returnvalue (Game|SpawnActorfromClass "/Game/_Game/BP/Enemies/Enemies/BP_EnemyEntity.BP_EnemyEntity_C" (Math|Transform|MakeTransform (Transformation|GetActorLocation) "0, 0, 0" "1.000000,1.000000,1.000000") "Undefined" "MultiplyWithRoot" 0 0))
  (return _returnvalue))

(fn CalculateBudget
  (params (Round :type Float%20%28double-precision%29))
  (return (+ (+ (* Round 8.0) 2e+01) (* (Math|Float|Floor (/ Round 1e+01)) 10))))

(fn PickEnemy
  (params (Round :type Float%20%28double-precision%29))
  (Utilities|Array|Clear (LocalVariables|GetAvailableEnemies))
  (LocalVariables|SetTotalWeight 0)
  (for _array_element (Variables|Default|GetEnemyPool)
    (if (and (<= (.MinRound (Utilities|Struct|BreakStructure_EnemyData _array_element)) Round) (<= (.Cost (Utilities|Struct|BreakStructure_EnemyData _array_element)) (Variables|Default|GetTempBudget)))
      (Utilities|Array|Add (LocalVariables|GetAvailableEnemies) _array_element)
      (switch Utilities|FlowControl|Switch|SwitchonE_WaveType (Variables|Default|GetCurrentWaveType%20)
        (:NewEnumerator0
          (LocalVariables|SetMultiplier 1.0))
        (:NewEnumerator1
          (if (<= (.Cost (Utilities|Struct|BreakStructure_EnemyData _array_element)) 15.0)
            (LocalVariables|SetMultiplier 2.0)
            (else
              (LocalVariables|SetMultiplier 0.5))))
        (:NewEnumerator2
          (if (>= (.Cost (Utilities|Struct|BreakStructure_EnemyData _array_element)) 25.0)
            (LocalVariables|SetMultiplier 2.0)
            (else
              (LocalVariables|SetMultiplier 0.5))))
        (:NewEnumerator3
          (if (.IsFast (Utilities|Struct|BreakStructure_EnemyData _array_element))
            (LocalVariables|SetMultiplier 2.0)
            (else
              (LocalVariables|SetMultiplier 0.7)))))
      (LocalVariables|SetTotalWeight (+ (* (Math|Integer|Clamp(Integer) (- (.MaxWeight (Utilities|Struct|BreakStructure_EnemyData _array_element)) (Math|Integer|Absolute(Integer) (- (Variables|Default|GetCurrentRound) (.PeakRound (Utilities|Struct|BreakStructure_EnemyData _array_element))))) 0 (.MaxWeight (Utilities|Struct|BreakStructure_EnemyData _array_element))) (LocalVariables|GetMultiplier)) (LocalVariables|GetTotalWeight)))))
  (if (> (LocalVariables|GetTotalWeight) 0)
    (LocalVariables|SetRandomWeight (Math|Random|RandomIntegerinRange 0 (- (LocalVariables|GetTotalWeight) 1)))
    (LocalVariables|SetRunningWeight 0)
    (for _array_element_2 (LocalVariables|GetAvailableEnemies)
      (switch Utilities|FlowControl|Switch|SwitchonE_WaveType (Variables|Default|GetCurrentWaveType%20)
        (:NewEnumerator0
          (LocalVariables|SetMultiplier 1.0))
        (:NewEnumerator1
          (if (<= (.Cost (Utilities|Struct|BreakStructure_EnemyData _array_element_2)) 15.0)
            (LocalVariables|SetMultiplier 2.0)
            (else
              (LocalVariables|SetMultiplier 0.5))))
        (:NewEnumerator2
          (if (>= (.Cost (Utilities|Struct|BreakStructure_EnemyData _array_element_2)) 25.0)
            (LocalVariables|SetMultiplier 2.0)
            (else
              (LocalVariables|SetMultiplier 0.5))))
        (:NewEnumerator3
          (if (.IsFast (Utilities|Struct|BreakStructure_EnemyData _array_element_2))
            (LocalVariables|SetMultiplier 2.0)
            (else
              (LocalVariables|SetMultiplier 0.7)))))
      (LocalVariables|SetRunningWeight (+ (* (Math|Integer|Clamp(Integer) (- (.MaxWeight (Utilities|Struct|BreakStructure_EnemyData _array_element_2)) (Math|Integer|Absolute(Integer) (- (Variables|Default|GetCurrentRound) (.PeakRound (Utilities|Struct|BreakStructure_EnemyData _array_element_2))))) 0 (.MaxWeight (Utilities|Struct|BreakStructure_EnemyData _array_element_2))) (LocalVariables|GetMultiplier)) (LocalVariables|GetRunningWeight)))
      (if (< (LocalVariables|GetRandomWeight) (LocalVariables|GetRunningWeight))
        (return _array_element_2 true)))
    (else
      (return "" false))))

(fn GetMoney
  (return 0))

(fn GetWLayout
  (return 0))