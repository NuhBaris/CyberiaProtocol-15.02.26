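; Player camera pawn for a map-selector view, panned along a clamped X axis with a fixed Y.
; On controller change it adds the input mapping, shows the cursor and creates the settings widget.
; Enhanced Input drives panning, while Tick overrides height to a large offset above the stored starting Z.
; Escape pauses the game and animates the settings widget; GetMoney is a stub returning zero.
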(event Input|EnhancedActionEvents|EnhancedInputActionIA_MapSelectorCameraMove
  (params (ActionValue :type Float%20%28double-precision%29) (ElapsedSeconds :type Float%20%28double-precision%29) (TriggeredSeconds :type Float%20%28double-precision%29) (InputAction :type Input%20Action%20Object%20Reference :default "/Game/_Game/BP/Input/Actions/IA_MapSelectorCameraMove.IA_MapSelectorCameraMove"))
  (bind _returnvalue (Utilities|Time|GetWorldDeltaSeconds))
  (bind _panspeed (Variables|Default|GetPanSpeed))
  ;[0.15 0.15 0.15 0.5] Camera
  (Transformation|SetActorLocation (Math|Vector|MakeVector (Math|Float|Clamp(Float) (.x (+ (+ (* (Transformation|GetActorRightVector) (* ActionValue _panspeed _returnvalue)) (* (Transformation|GetActorForwardVector) (* ActionValue _panspeed _returnvalue))) (Transformation|GetActorLocation))) (Variables|Default|GetMapMin) (Variables|Default|GetMapMax2)) 2.37e+03 22688.0) false false))

(event EventControllerChanged
  (params (OldController :type Controller%20Object%20Reference) (NewController :type Controller%20Object%20Reference))
  (bind _returnvalue (Game|GetPlayerController 0))
  ;[0.15 0.15 0.15 0.5] Beginplay
  (bind _asplayer_controller (Utilities|Casting|CastToPlayerController NewController))
  (Input|AddMappingContext (PlayerController|LocalPlayerSubsystems|GetEnhancedInputLocalPlayerSubsystem _asplayer_controller) "/Game/_Game/BP/Input/IMC_Default.IMC_Default" 1 "(bIgnoreAllPressedKeysUntilRelease=True,bForceImmediately=False,bNotifyUserSettings=False)")
  (Variables|/Script/Engine.PlayerController|SetbShowMouseCursor _returnvalue true)
  (Input|SetInputModeGameandUI _returnvalue 0 "DoNotLock" true false)
  (Variables|Default|SetZ (.z (Transformation|GetActorLocation)))
  (bind _returnvalue_2 (UserInterface|CreateWidget "/Game/_Game/BP/Widgets/W_WrappedSettings.W_WrappedSettings_C"))
  (bind _output_get (Variables|Default|SetWrappedSetting _returnvalue_2))
  (UserInterface|Viewport|AddtoViewport _output_get 0))

(event EventTick
  (params (DeltaSeconds :type Float%20%28single-precision%29))
  (bind _returnvalue (Transformation|GetActorLocation))
  ;[0.15 0.15 0.15 0.5] Tick
  (Transformation|SetActorLocation (Math|Vector|MakeVector (.x _returnvalue) (.y _returnvalue) (+ (Variables|Default|GetZ) 9.5e+04)) false false))

(event Input|KeyboardEvents|Escape
  (params (Key :type Key%20Structure))
  (bind _wrappedsetting (Variables|Default|GetWrappedSetting))
  ;[0.15 0.15 0.15 0.5] Esc
  (:Pressed
    (Game|SetGamePaused true)
    (UserInterface|Animation|PlayAnimation _wrappedsetting (Variables|/Game/_Game/BP/Widgets/W_WrappedSettings.W_WrappedSettings_C|Getsettinganim _wrappedsetting) 0.0 1 "Forward" 1.0 false)
    (Variables|/Game/_Game/BP/Widgets/W_WrappedSettings.W_WrappedSettings_C|Setasagida _wrappedsetting false)))

(fn ConstructionScript)

(fn GetMoney
  (return 0))