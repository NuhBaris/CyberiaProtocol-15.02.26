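; BP_Bullet is a tower-fired projectile that homes in on an assigned enemy.
; On BeginPlay it gets the mesh from TargetEnemy and sets it as the ProjectileMovement homing target.
; When its Sphere overlaps any BPI_Enemy actor and Tower is valid, it sends BulletHitMessage to the Tower, then destroys its movement component and itself.
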(event OnComponentBeginOverlap(Sphere)
  (params (OverlappedComponent :type Primitive%20Component%20Object%20Reference) (OtherActor :type Actor%20Object%20Reference) (OtherComp :type Primitive%20Component%20Object%20Reference) (OtherBodyIndex :type Integer) (bFromSweep :type Boolean) (SweepResult :type Hit%20Result%20Structure%20%28by%20ref%29))
  (bind _tower (Variables|Default|GetTower))
  (if (Utilities|DoesObjectImplementInterface OtherActor "/Game/_Game/BP/Frameworks/BPI_Enemy.BPI_Enemy_C")
    (Utilities|IsValid _tower
      (:Is%20Valid
        (Class|BPITowers|BulletHit(Message) _tower)
        (Components|DestroyComponent (Variables|Default|GetProjectileMovement))
        (Actor|DestroyActor)))))

(event EventBeginPlay
  (bind _targetenemy (Variables|Default|GetTargetEnemy))
  (Utilities|IsValid _targetenemy
    (:Is%20Valid
      (bind _mesh (Class|BPIEnemy|GetEnemyMesh(Message) _targetenemy))
      (Variables|/Script/Engine.ProjectileMovementComponent|SetHomingTargetComponent (Variables|Default|GetProjectileMovement) _mesh))))

(fn ConstructionScript)