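; BP_WanderingThings is an actor that moves its mesh along a spline using a timeline, blending rotation toward the spline's direction.
; Movement starts at BeginPlay unless IsFirst is set.
; It also binds to the Stages event of the W_MainMenu widget on BP_Computer.
; That event, once only, sets the mesh's height, waits, animates it vertically at the spline's end, then plays the path timeline.
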(event Custom|StagesEvents
  (bind _spline (Variables|Default|GetSpline))
  (bind _spline_2 (Variables|Default|GetSpline))
  (bind _sm (Variables|Default|GetSM))
  (bind _sm_2 (Variables|Default|GetSM))
  (bind _sm_3 (Variables|Default|GetSM))
  (bind _returnvalue (Transformation|GetWorldLocation _sm))
  (bind _returnvalue_2 (Spline|GetSplineLength _spline))
  (bind _returnvalue_3 (Spline|GetLocationatDistanceAlongSpline _spline _returnvalue_2 "World"))
  (Utilities|FlowControl|DoOnce false
    (:Completed
      (Transformation|SetWorldLocation _sm (Math|Vector|MakeVector (.x _returnvalue) (.y _returnvalue) (Variables|Default|GetLoc1)) false false)
      (Variables|Default|SetIsFirst false)
      (Utilities|FlowControl|Delay (Variables|Default|GetDuration))
      (bind _a (Timeline|Timeline_0 Play)
        (:Update
          (Transformation|SetWorldLocation _sm_3 (Math|Vector|MakeVector (.x _returnvalue_3) (.y _returnvalue_3) (Math|Float|Lerp (Variables|Default|GetLoc1) (Variables|Default|GetLoc2) _a)) false false)
          (Transformation|SetWorldRotation _sm_3 (Spline|GetRotationatDistanceAlongSpline _spline _returnvalue_2 "World") false false))
        (:Finished
          (bind _a_2 (Timeline|Timeline Play)
            (:Update
              (Transformation|SetWorldTransform _sm_2 (Math|Transform|MakeTransform (Spline|GetLocationatDistanceAlongSpline _spline_2 (Math|Float|Lerp 0.0 (Spline|GetSplineLength (Variables|Default|GetSpline)) _a_2) "World") (Math|Rotator|Lerp(Rotator) (Transformation|GetWorldRotation _sm_2) (Spline|GetRotationatDistanceAlongSpline _spline_2 (Math|Float|Lerp 0.0 (Spline|GetSplineLength (Variables|Default|GetSpline)) _a_2) "World") _a_2) "1.000000,1.000000,1.000000") false false))))))))

(event EventBeginPlay
  (bind _spline (Variables|Default|GetSpline))
  (bind _sm (Variables|Default|GetSM))
  (bind _outactors (Actor|GetAllActorsOfClass "/Game/_Game/BP/BP_Computer.BP_Computer_C"))
  (bind _asw_main_menu (Utilities|Casting|CastToW_MainMenu (UserInterface|GetWidget (Variables|/Game/_Game/BP/BP_Computer.BP_Computer_C|GetWidgetA (Utilities|Array|Get(acopy) _outactors)))))
  (EventDispatchers|BindEventtoStages _asw_main_menu (delegate Custom|StagesEvents))
  (if (not (Variables|Default|GetIsFirst))
    (bind _a (Timeline|Timeline Play)
      (:Update
        (Transformation|SetWorldTransform _sm (Math|Transform|MakeTransform (Spline|GetLocationatDistanceAlongSpline _spline (Math|Float|Lerp 0.0 (Spline|GetSplineLength (Variables|Default|GetSpline)) _a) "World") (Math|Rotator|Lerp(Rotator) (Transformation|GetWorldRotation _sm) (Spline|GetRotationatDistanceAlongSpline _spline (Math|Float|Lerp 0.0 (Spline|GetSplineLength (Variables|Default|GetSpline)) _a) "World") _a) "1.000000,1.000000,1.000000") false false)))))

(fn ConstructionScript)