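; BP_Robo is an actor that moves its Hoverboard component along a spline once play begins.
; A Timeline started on BeginPlay maps its alpha to distance along the spline, setting world location from that point each update.
; Rotation blends from the board's current rotation toward the spline's by the same alpha, keeping scale unchanged.
; Enemy speed, mesh, health and length getters are stubs returning zero or empty values.
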(event EventBeginPlay
  (bind _hoverboard (Variables|Default|Gethoverboard))
  (bind _spline (Variables|Default|GetSpline))
  (Utilities|FlowControl|Sequence
    (:then_0
      (bind _a (Timeline|Timeline PlayFromStart)
        (:Update
          (Transformation|SetWorldTransform _hoverboard (Math|Transform|MakeTransform (Math|Vector|MakeVector (.x (Spline|GetLocationatDistanceAlongSpline _spline (Math|Float|Lerp 0.0 (Spline|GetSplineLength (Variables|Default|GetSpline)) _a) "World")) (.y (Spline|GetLocationatDistanceAlongSpline _spline (Math|Float|Lerp 0.0 (Spline|GetSplineLength (Variables|Default|GetSpline)) _a) "World")) (.z (Spline|GetLocationatDistanceAlongSpline _spline (Math|Float|Lerp 0.0 (Spline|GetSplineLength (Variables|Default|GetSpline)) _a) "World"))) (Math|Rotator|MakeRotator (.roll (Math|Rotator|Lerp(Rotator) (Transformation|GetWorldRotation _hoverboard) (Spline|GetRotationatDistanceAlongSpline _spline (Math|Float|Lerp 0.0 (Spline|GetSplineLength (Variables|Default|GetSpline)) _a) "World") _a true)) (.pitch (Math|Rotator|Lerp(Rotator) (Transformation|GetWorldRotation _hoverboard) (Spline|GetRotationatDistanceAlongSpline _spline (Math|Float|Lerp 0.0 (Spline|GetSplineLength (Variables|Default|GetSpline)) _a) "World") _a true)) (.yaw (Math|Rotator|Lerp(Rotator) (Transformation|GetWorldRotation _hoverboard) (Spline|GetRotationatDistanceAlongSpline _spline (Math|Float|Lerp 0.0 (Spline|GetSplineLength (Variables|Default|GetSpline)) _a) "World") _a true))) (Transformation|GetWorldScale _hoverboard)) false false))))))

(fn ConstructionScript)

(fn GetEnemySpeed
  (return 0.0))

(fn GetEnemyMesh
  (return 0))

(fn GetEnemyHealth
  (return 0.0 0.0))

(fn GetLength
  (return 0.0 0.0))