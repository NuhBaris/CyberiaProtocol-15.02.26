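; Tower defense player controller handling tower placement, money, range display and enemy wave start, plus a money cheat key.
; StartPlacing spawns a ghost preview and a far-off tower instance that supplies class and cost.
; A looping timer moves the ghost under the cursor, snapping to interface-implementing actors and showing ranges.
; Clicks build on free BP_Grid tiles and report money to the pawn, or toggle tower ranges outside placement.
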(event Custom|Ghost
  (bind _returnvalue (Game|GetPlayerController 0))
  (bind _hitresult (Game|Player|GetHitResultUnderCursorbyChannel "TraceTypeQuery1" true))
  (bind _ghosttower (Variables|Default|GetGhostTower))
  (bind (_locationx _locationy) (Game|Player|GetMousePosition _returnvalue))
  (bind _hitactor (Collision|BreakHitResult _hitresult))
  (bind _ranges (Variables|/Game/_Protocol/BP/Towers/BP_TowerBase.BP_TowerBase_C|GetRanges _ghosttower))
  (bind _returnvalue_2 (Transformation|GetActorLocation _hitactor))
  (bind (_worldposition _worlddirection) (Class|GameplayStatics|DeprojectScreentoWorld _returnvalue (Math|Vector2D|MakeVector2D _locationx _locationy)))
  ;[0.15 0.15 0.15 0.5] Beginplay / Ghost
  (if (or (Variables|Default|GetbIsPlacingTower%20%20) (Utilities|IsValid (Variables|Default|GetGhostTower)))
    (if (Utilities|DoesObjectImplementInterface _hitactor "/Game/_Protocol/BP/Frameworks/BP_GeneralInterface.BP_GeneralInterface_C")
      (Transformation|SetActorLocation _ghosttower (Math|Vector|MakeVector (- (.x _returnvalue_2) (Variables|Default|GetSpawnSubX)) (- (.y _returnvalue_2) (Variables|Default|GetSpawnSubY)) 4755.385304) false false)
      (for _array_element _ranges
        (Rendering|SetVisibility _array_element true false))
      (else
        (Transformation|SetActorLocation _ghosttower (+ _worldposition (* _worlddirection 2e+04)) false false)
        (for _array_element_2 _ranges
          (Rendering|SetVisibility _array_element_2 false false))))))

(event Custom|StartPlacing
  (params (TowerName :type String))
  ;[0.15 0.15 0.15 0.5] StartPlacing (Custom Event)
  (Variables|Default|SetbIsPlacingTower%20%20 true)
  (switch string TowerName
    (:Minigun
      (bind _returnvalue (Game|SpawnActorfromClass "/Game/_Protocol/BP/Towers/BP_GhostByteBlaster.BP_GhostByteBlaster_C" (Math|Transform|MakeTransform "0, 0, 0" "0, 0, 0" "1.000000,1.000000,1.000000") "Undefined" "MultiplyWithRoot" 0 0))
      (bind _returnvalue_2 (Game|SpawnActorfromClass "/Game/_Protocol/BP/Towers/BP_TowerByteBlaster.BP_TowerByteBlaster_C" (Math|Transform|MakeTransform "0.000000,0.000000,1000000.000000" "0, 0, 0" "1.000000,1.000000,1.000000") "Undefined" "MultiplyWithRoot" 0 0))
      (Variables|Default|SetGhostTower _returnvalue)
      (Variables|Default|SetSelectedTower _returnvalue_2))
    (:Support
      (bind _returnvalue_3 (Game|SpawnActorfromClass "/Game/_Protocol/BP/Towers/BP_GhostSupport.BP_GhostSupport_C" (Math|Transform|MakeTransform "0, 0, 0" "0, 0, 0" "1.000000,1.000000,1.000000") "Undefined" "MultiplyWithRoot" 0 0))
      (bind _returnvalue_4 (Game|SpawnActorfromClass "/Game/_Protocol/BP/Towers/BP_TowerSupport.BP_TowerSupport_C" (Math|Transform|MakeTransform "0.000000,0.000000,1000000.000000" "0, 0, 0" "1.000000,1.000000,1.000000") "Undefined" "MultiplyWithRoot" 0 0))
      (Variables|Default|SetGhostTower _returnvalue_3)
      (Variables|Default|SetSelectedTower _returnvalue_4))
    (:Roketatar
      (bind _returnvalue_5 (Game|SpawnActorfromClass "/Game/_Protocol/BP/Towers/BP_GhostMissileLauncher.BP_GhostMissileLauncher_C" (Math|Transform|MakeTransform "0, 0, 0" "0, 0, 0" "1.000000,1.000000,1.000000") "Undefined" "MultiplyWithRoot" 0 0))
      (bind _returnvalue_6 (Game|SpawnActorfromClass "/Game/_Protocol/BP/Towers/BP_TowerMissileLauncher.BP_TowerMissileLauncher_C" (Math|Transform|MakeTransform "0.000000,0.000000,1000000.000000" "0, 0, 0" "1.000000,1.000000,1.000000") "Undefined" "MultiplyWithRoot" 0 0))
      (Variables|Default|SetGhostTower _returnvalue_5)
      (Variables|Default|SetSelectedTower _returnvalue_6))
    (:Tesla
      (bind _returnvalue_7 (Game|SpawnActorfromClass "/Game/_Protocol/BP/Towers/BP_GhostSurge.BP_GhostSurge_C" (Math|Transform|MakeTransform "0, 0, 0" "0, 0, 0" "1.000000,1.000000,1.000000") "Undefined" "MultiplyWithRoot" 0 0))
      (bind _returnvalue_8 (Game|SpawnActorfromClass "/Game/_Protocol/BP/Towers/BP_TowerSurge.BP_TowerSurge_C" (Math|Transform|MakeTransform "0.000000,0.000000,1000000.000000" "0, 0, 0" "1.000000,1.000000,1.000000") "Undefined" "MultiplyWithRoot" 0 0))
      (Variables|Default|SetGhostTower _returnvalue_7)
      (Variables|Default|SetSelectedTower _returnvalue_8))))

(event EventBeginPlay
  ;[0.15 0.15 0.15 0.5] Beginplay / Ghost
  (bind _money (Class|BPGeneralInterface|GetMoney(Message) (Game|Player|GetPlayerPawn 0)))
  (Variables|Default|SetMoney _money)
  (Utilities|Time|SetTimerbyEvent (delegate Custom|Ghost) 0.01 true))

(event EventTowerButtonClicked
  ;[0.15 0.15 0.15 0.5] TowerDetails
  (Utilities|IsValid (Variables|Default|GetLastClickedTower)
    (:Is%20Valid
      (Default|ShowHideRange (Variables|Default|GetLastClickedTower) false)
      (Variables|Default|SetLastClickedTower 0))))

(event Input|MouseEvents|LeftMouseButton
  (params (Key :type Key%20Structure))
  (bind _ghosttower (Variables|Default|GetGhostTower))
  (bind _selectedtower (Variables|Default|GetSelectedTower))
  (:Pressed
    (if (Variables|Default|GetbIsPlacingTower%20%20)
      ;[0.15 0.15 0.15 0.5] Placement
      (bind _asbp_grid (Utilities|Casting|CastToBP_Grid (.hitactor (.HitResult (Game|Player|GetHitResultUnderCursorbyChannel "TraceTypeQuery1" true)))))
      (Variables|Default|SetHoveredTile _asbp_grid)
      (if (and (not (Variables|/Game/_Protocol/BP/BP_Grid.BP_Grid_C|GetCantPlaceTower (Variables|Default|GetHoveredTile))) (not (Variables|/Game/_Protocol/BP/BP_Grid.BP_Grid_C|GetIsOccupied (Variables|Default|GetHoveredTile))))
        (Game|SpawnActorfromClass (Utilities|GetClass _selectedtower) (Math|Transform|MakeTransform (Math|Vector|MakeVector (- (.x (Transformation|GetActorLocation (Variables|Default|GetHoveredTile))) (Variables|Default|GetSpawnSubX)) (- (.y (Transformation|GetActorLocation (Variables|Default|GetHoveredTile))) (Variables|Default|GetSpawnSubY)) 4755.385304) "0, 0, 0" "1.000000,1.000000,1.000000") "Undefined" "MultiplyWithRoot" 0 0)
        (bind _output_get (Variables|Default|SetMoney (- (Variables|Default|GetMoney) (.Cost (Utilities|Struct|BreakStructure_TowerBase (Variables|/Game/_Protocol/BP/Towers/BP_TowerBase.BP_TowerBase_C|GetStructure_Base _selectedtower))))))
        (Class|BPGeneralInterface|MoneyChanged(Message) (Game|Player|GetPlayerPawn 0) _output_get)
        (Variables|/Game/_Protocol/BP/BP_Grid.BP_Grid_C|SetIsOccupied (Variables|Default|GetHoveredTile) true)
        (Variables|Default|SetbIsPlacingTower%20%20 false)
        (if (Utilities|IsValid _ghosttower)
          (Actor|DestroyActor _ghosttower)))
      (else
        ;[0.15 0.15 0.15 0.5] TowerDetails
        (bind _asbp_tower_base (Utilities|Casting|CastToBP_TowerBase (.hitactor (.HitResult (Game|Player|GetHitResultUnderCursorbyChannel "TraceTypeQuery1" true))))
          (:then
            (Utilities|IsValid (Variables|Default|GetLastClickedTower)
              (:Is%20Valid
                (if (not (== (Variables|/Game/_Protocol/BP/Towers/BP_TowerBase.BP_TowerBase_C|GetTower _asbp_tower_base) (Variables|Default|GetLastClickedTower)))
                  (Default|ShowHideRange (Variables|Default|GetLastClickedTower) false)
                  (Default|ShowHideRange (Variables|/Game/_Protocol/BP/Towers/BP_TowerBase.BP_TowerBase_C|GetTower _asbp_tower_base) true)
                  (Variables|Default|SetLastClickedTower (Variables|/Game/_Protocol/BP/Towers/BP_TowerBase.BP_TowerBase_C|GetTower _asbp_tower_base))))
              (:Is%20Not%20Valid
                (Variables|Default|SetLastClickedTower (Variables|/Game/_Protocol/BP/Towers/BP_TowerBase.BP_TowerBase_C|GetTower _asbp_tower_base))
                (Default|ShowHideRange (Variables|/Game/_Protocol/BP/Towers/BP_TowerBase.BP_TowerBase_C|GetTower _asbp_tower_base) true))))
          (:CastFailed
            (Utilities|IsValid (Variables|Default|GetLastClickedTower)
              (:Is%20Valid
                (Default|ShowHideRange (Variables|Default|GetLastClickedTower) false)
                (Variables|Default|SetLastClickedTower 0)))))))))

(event Input|MouseEvents|MiddleMouseButton
  (params (Key :type Key%20Structure))
  (bind _ghosttower (Variables|Default|GetGhostTower))
  ;[0.15 0.15 0.15 0.5] Cancel
  (:Pressed
    (if (Utilities|IsValid _ghosttower)
      (Actor|DestroyActor _ghosttower)
      (Variables|Default|SetbIsPlacingTower%20%20 false))))

(event Input|KeyboardEvents|SpaceBar
  (params (Key :type Key%20Structure))
  ;[0.15 0.15 0.15 0.5] Space
  (:Pressed
    (bind _outactors (Actor|GetAllActorsOfClass "/Game/_Protocol/BP/BP_EnemySpawner.BP_EnemySpawner_C"))
    (Default|NextWave (Utilities|Array|Get(acopy) _outactors))))

(event Input|KeyboardEvents|5
  (params (Key :type Key%20Structure))
  ;[0.15 0.15 0.15 0.5] Placement
  (:Pressed
    (Variables|Default|SetMoney (+ (Variables|Default|GetMoney) 500))
    (Class|BPGeneralInterface|MoneyChanged(Message) (Game|Player|GetPlayerPawn 0) (+ (Variables|Default|GetMoney) 500))))

(fn ConstructionScript)

(fn GetMoney
  (return 0))

(fn MoneyChanged
  (params (Money :type Integer))
  (return))