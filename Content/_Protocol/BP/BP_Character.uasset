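; Player character acting as a height-locked map camera that also owns the HUD and current money value.
; Enhanced Input drives yaw rotation and drag-to-pan within map bounds, while Tick holds Z constant.
; R resets the view and T snaps yaw to the nearest right angle via SetRotationFlatness.
; It creates the layout and settings widgets, pauses into animated settings on Escape, and forwards money changes to the layout.
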(event Input|EnhancedActionEvents|EnhancedInputActionIA_CamDrag
  (params (ActionValue :type Boolean) (ElapsedSeconds :type Float%20%28double-precision%29) (TriggeredSeconds :type Float%20%28double-precision%29) (InputAction :type Input%20Action%20Object%20Reference :default "/Game/_Protocol/BP/Input/Actions/IA_CamDrag.IA_CamDrag"))
  (bind _returnvalue (Game|GetPlayerController 0))
  ;[0.15 0.15 0.15 0.5] Camera
  ;;[0.15 0.15 0.15 0.5] Drag
  (:Triggered
    (Variables|Default|SetbDragging true)
    (Variables|/Script/Engine.PlayerController|SetbShowMouseCursor _returnvalue false))
  (:Completed
    (Variables|Default|SetbDragging false)
    (Variables|/Script/Engine.PlayerController|SetbShowMouseCursor _returnvalue true)))

(event Input|EnhancedActionEvents|EnhancedInputActionIA_CamPan
  (params (ActionValue :type Vector%202D%20Structure) (ElapsedSeconds :type Float%20%28double-precision%29) (TriggeredSeconds :type Float%20%28double-precision%29) (InputAction :type Input%20Action%20Object%20Reference :default "/Game/_Protocol/BP/Input/Actions/IA_CamPan.IA_CamPan"))
  (bind _returnvalue (Transformation|GetActorRightVector))
  (bind _returnvalue_2 (Transformation|GetActorForwardVector))
  (bind _returnvalue_3 (Transformation|GetActorLocation))
  (bind _returnvalue_4 (Utilities|Time|GetWorldDeltaSeconds))
  (bind _panspeed (Variables|Default|GetPanSpeed))
  (bind _returnvalue_5 (* (.y ActionValue) _panspeed _returnvalue_4))
  (bind _returnvalue_6 (* (.x ActionValue) _panspeed _returnvalue_4))
  (bind _returnvalue_7 (* _returnvalue_2 _returnvalue_5))
  (bind _returnvalue_8 (* _returnvalue _returnvalue_6))
  (bind _returnvalue_9 (+ _returnvalue_8 _returnvalue_7))
  (bind _returnvalue_10 (+ _returnvalue_9 _returnvalue_3))
  ;[0.15 0.15 0.15 0.5] Camera
  ;;[0.15 0.15 0.15 0.5] Pan
  (if (Variables|Default|GetbDragging)
    (Transformation|SetActorLocation (Math|Vector|MakeVector (Math|Float|Clamp(Float) (.x _returnvalue_10) (.x (Variables|Default|GetMapMin)) (.x (Variables|Default|GetMapMax))) (Math|Float|Clamp(Float) (.y _returnvalue_10) (.y (Variables|Default|GetMapMin)) (.y (Variables|Default|GetMapMax))) 23815.357478) false false)))

(event Input|EnhancedActionEvents|EnhancedInputActionIA_CamRot
  (params (ActionValue :type Vector%202D%20Structure) (ElapsedSeconds :type Float%20%28double-precision%29) (TriggeredSeconds :type Float%20%28double-precision%29) (InputAction :type Input%20Action%20Object%20Reference :default "/Game/_Protocol/BP/Input/Actions/IA_CamRot.IA_CamRot"))
  ;[0.15 0.15 0.15 0.5] Camera
  ;;[0.15 0.15 0.15 0.5] Rotation
  (Pawn|Input|AddControllerYawInput (* (.x ActionValue) (Variables|Default|GetRotationSpeed) (Utilities|Time|GetWorldDeltaSeconds) 9e+01)))

(event EventBeginPlay
  (bind _returnvalue (Game|GetPlayerController 0))
  ;[0.15 0.15 0.15 0.5] Beginplay
  (bind _returnvalue_2 (UserInterface|CreateWidget "/Game/_Protocol/BP/Widgets/W_Layout.W_Layout_C"))
  (bind _output_get (Variables|Default|SetWLayout _returnvalue_2))
  (UserInterface|Viewport|AddtoViewport _output_get 0)
  (Variables|/Script/Engine.PlayerController|SetbShowMouseCursor _returnvalue true)
  (Variables|Default|SetSavedWorldRotation (Transformation|GetWorldRotation (Variables|Collision|GetCapsuleComponent)))
  (Input|SetInputModeGameandUI _returnvalue (Variables|Default|GetWLayout) "DoNotLock" true false))

(event EventControllerChanged
  (params (OldController :type Controller%20Object%20Reference) (NewController :type Controller%20Object%20Reference))
  ;[0.15 0.15 0.15 0.5] Beginplay
  (bind _asplayer_controller (Utilities|Casting|CastToPlayerController NewController))
  (Input|AddMappingContext (PlayerController|LocalPlayerSubsystems|GetEnhancedInputLocalPlayerSubsystem _asplayer_controller) "/Game/_Protocol/BP/Input/IMC_Default.IMC_Default" 1 "(bIgnoreAllPressedKeysUntilRelease=True,bForceImmediately=False,bNotifyUserSettings=False)")
  (bind _returnvalue (UserInterface|CreateWidget "/Game/_Protocol/BP/Widgets/W_WrappedSettings.W_WrappedSettings_C"))
  (bind _output_get (Variables|Default|SetAsWrappedSettings _returnvalue))
  (UserInterface|Viewport|AddtoViewport _output_get 0)
  (Variables|Default|SetZ (.z (Transformation|GetActorLocation))))

(event EventTick
  (params (DeltaSeconds :type Float%20%28single-precision%29))
  (bind _returnvalue (Transformation|GetActorLocation))
  ;[0.15 0.15 0.15 0.5] Tick
  (Transformation|SetActorLocation (Math|Vector|MakeVector (.x _returnvalue) (.y _returnvalue) (Variables|Default|GetZ)) false false))

(event EventMoneyChanged
  (params (Money :type Integer))
  (bind _output_get (Variables|Default|SetCurrentMoney Money))
  (Default|MoneyChanged (Variables|Default|GetWLayout) _output_get))

(event Input|KeyboardEvents|R
  (params (Key :type Key%20Structure :default "None"))
  ;[0.15 0.15 0.15 0.5] Camera
  ;;[0.15 0.15 0.15 0.5] Rotation
  (:Pressed
    (Transformation|SetActorLocation (Math|Vector|MakeVector -5430.858887 1714.484009 23815.357422) false false)
    (Pawn|SetControlRotation (Pawn|GetController) (Math|Rotator|MakeRotator 0.0 0.0 0.0))))

(event Input|KeyboardEvents|Escape
  (params (Key :type Key%20Structure :default "None"))
  (bind _aswrappedsettings (Variables|Default|GetAsWrappedSettings))
  ;[0.15 0.15 0.15 0.5] Escape
  (:Pressed
    (Default|ClosewithEscape (Variables|Default|GetWLayout))
    (Game|SetGamePaused true)
    (UserInterface|Animation|PlayAnimation _aswrappedsettings (Variables|/Game/_Protocol/BP/Widgets/W_WrappedSettings.W_WrappedSettings_C|Getsettinganim _aswrappedsettings) 0.0 1 "Forward" 1.0 false)
    (Variables|/Game/_Protocol/BP/Widgets/W_WrappedSettings.W_WrappedSettings_C|Setasagida _aswrappedsettings false)))

(event Input|KeyboardEvents|T
  (params (Key :type Key%20Structure :default "None"))
  ;[0.15 0.15 0.15 0.5] Camera
  ;;[0.15 0.15 0.15 0.5] Rotation
  (:Pressed
    (bind _resultrotation (Utilities|SetRotationFlatness (.yaw (Transformation|GetWorldRotation (Variables|Collision|GetCapsuleComponent))))
      (:End
        (Pawn|SetControlRotation (Pawn|GetController) (Math|Rotator|MakeRotator 0.0 0.0 _resultrotation))))))

(fn ConstructionScript)

(fn GetMoney
  (return (Variables|Default|GetCurrentMoney)))