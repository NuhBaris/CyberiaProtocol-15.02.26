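; BP_Yol is a spline-driven path actor that lays a deformable mesh along an editable spline.
; Its construction script destroys existing spline mesh components, then adds one Movable SM_Yol segment with the M_Path material for each pair of consecutive spline points.
; Each segment bends along its X axis, using the local-space locations and tangents of its two points so the path follows the curve continuously.
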(fn ConstructionScript
  (bind _spline (Variables|Default|GetSpline))
  (for _array_element (Actor|GetComponentsByClass "/Script/Engine.SplineMeshComponent")
    (Components|DestroyComponent _array_element))
  (for _index (range 0 (- (Spline|GetNumberOfSplinePoints (Variables|Default|GetSpline)) 2))
    (bind _returnvalue (AddComponent|AddSplineMeshComponent false))
    (Components|StaticMesh|SetStaticMesh _returnvalue "/Game/_Protocol/Levels/_GENERATED/nbarisd/SM_Yol.SM_Yol")
    (SplineMesh|SetForwardAxis _returnvalue "X" true)
    (Rendering|Material|SetMaterial _returnvalue 0 "/Game/_Protocol/Materials/M_Path.M_Path")
    (Transformation|SetMobility _returnvalue "Movable")
    (SplineMesh|SetStartandEnd _returnvalue (Spline|GetLocationatSplinePoint _spline _index "Local") (Spline|GetTangentatSplinePoint _spline _index "Local") (Spline|GetLocationatSplinePoint _spline (+ _index 1) "Local") (Spline|GetTangentatSplinePoint _spline (+ _index 1) "Local") true :!class /Script/Engine.SplineMeshComponent)))