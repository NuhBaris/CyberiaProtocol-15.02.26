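; Enemy wave spawner that increments the round on NextWave and spawns enemies at its own location within a round-scaled budget.
; CalculateBudget grows linearly with a step bonus every ten rounds.
; PickEnemy makes a weighted random choice from EnemyPool entries unlocked by MinRound.
; SpawnNextEnemy re-calls itself after a short delay, subtracting each enemy's cost until the budget runs out, so the last pick can overspend.
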(event Custom|SpawnWave
  (bind _bugdet (CallFunction|CalculateBudget (Math|Conversions|ToFloat(Integer) (Variables|Default|GetCurrentRound))))
  (Variables|Default|SetCurrentBudget (Math|Float|Truncate _bugdet))
  (Utilities|FlowControl|Delay 0.2)
  (CallFunction|SpawnNextEnemy))

(event Custom|SpawnNextEnemy
  (if (> (Variables|Default|GetCurrentBudget) 0)
    (bind (_enemydata _isvalid) (CallFunction|PickEnemy (Math|Conversions|ToFloat(Integer) (Variables|Default|GetCurrentRound))))
    (if _isvalid
      (Game|SpawnActorfromClass (.EnemyClass (Utilities|Struct|BreakStructure_EnemyData _enemydata)) (Math|Transform|MakeTransform (Transformation|GetActorLocation) "0, 0, 0" "1.000000,1.000000,1.000000") "Undefined" "MultiplyWithRoot" 0 0)
      (Variables|Default|SetCurrentBudget (Math|Float|Truncate (- (Variables|Default|GetCurrentBudget) (.Cost (Utilities|Struct|BreakStructure_EnemyData _enemydata)))))
      (Utilities|FlowControl|Delay 0.7)
      (CallFunction|SpawnNextEnemy))))

(event EventNextWave
  (Variables|Default|SetCurrentRound (+ (Variables|Default|GetCurrentRound) 1))
  (CallFunction|SpawnWave))

(fn ConstructionScript)

(fn CreateEnemy
  (bind _returnvalue (Game|SpawnActorfromClass "/Game/_Protocol/BP/Enemies/BP_EnemyEntity.BP_EnemyEntity_C" (Math|Transform|MakeTransform (Transformation|GetActorLocation) "0, 0, 0" "1.000000,1.000000,1.000000") "Undefined" "MultiplyWithRoot" 0 0))
  (return _returnvalue))

(fn CalculateBudget
  (params (Round :type Float%20%28double-precision%29))
  (return (+ (+ (* Round 8.0) 2e+01) (* (Math|Float|Floor (/ Round 1e+01)) 10))))

(fn PickEnemy
  (params (Round :type Float%20%28double-precision%29))
  (Utilities|Array|Clear (LocalVariables|GetAvailableEnemies))
  (LocalVariables|SetTotalWeight 0)
  (for _array_element (Variables|Default|GetEnemyPool)
    (if (<= (.MinRound (Utilities|Struct|BreakStructure_EnemyData _array_element)) Round)
      (Utilities|Array|Add (LocalVariables|GetAvailableEnemies) _array_element)
      (LocalVariables|SetTotalWeight (Math|Float|Truncate (+ (.Weight (Utilities|Struct|BreakStructure_EnemyData _array_element)) (LocalVariables|GetTotalWeight))))))
  (if (> (LocalVariables|GetTotalWeight) 0)
    (LocalVariables|SetRandomWeight (Math|Random|RandomIntegerinRange 0 (- (LocalVariables|GetTotalWeight) 1)))
    (LocalVariables|SetRunningWeight 0)
    (for _array_element_2 (LocalVariables|GetAvailableEnemies)
      (LocalVariables|SetRunningWeight (+ (.Weight (Utilities|Struct|BreakStructure_EnemyData _array_element_2)) (LocalVariables|GetRunningWeight)))
      (if (< (LocalVariables|GetRandomWeight) (LocalVariables|GetRunningWeight))
        (return _array_element_2 true)))
    (else
      (return "" false))))

(fn GetMoney
  (return 0))