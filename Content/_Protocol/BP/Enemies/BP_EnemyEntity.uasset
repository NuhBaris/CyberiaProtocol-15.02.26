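; BP_EnemyEntity is an enemy actor that travels along the level's spline path while steadily losing health.
; On BeginPlay it starts a fast looping timer and takes the first BP_EnemyPath found in the level.
; Each tick of that timer drains Health, advances a clamped spline distance by Speed, and snaps the actor's location and rotation to that point.
; Nothing here handles zero health or reaching the path's end.
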(event Custom|CustomEvent
  (bind _enemypath (Variables|Default|GetEnemyPath))
  (bind _spline_enemypath (Variables|/Game/_Protocol/BP/BP_EnemyPath.BP_EnemyPath_C|GetSpline_EnemyPath _enemypath))
  (Variables|Default|SetHealth (- (Variables|Default|GetHealth) 0.1))
  (bind _output_get (Variables|Default|SetDistanceOnSpline (Math|Float|Clamp(Float) (+ (Variables|Default|GetDistanceOnSpline) (Variables|Default|GetSpeed)) 0.0 (Spline|GetSplineLength _spline_enemypath))))
  (Transformation|SetActorTransform (Math|Transform|MakeTransform (Spline|GetLocationatDistanceAlongSpline _spline_enemypath _output_get "World") (Spline|GetRotationatDistanceAlongSpline _spline_enemypath _output_get "World") "1.000000,1.000000,1.000000")))

(event EventBeginPlay
  (Utilities|Time|SetTimerbyEvent (delegate Custom|CustomEvent) 0.02 true)
  (bind _outactors (Actor|GetAllActorsOfClass "/Game/_Protocol/BP/BP_EnemyPath.BP_EnemyPath_C"))
  (Variables|Default|SetEnemyPath (Utilities|Array|Get(acopy) _outactors)))

(fn ConstructionScript
  (|CallParentFunction))