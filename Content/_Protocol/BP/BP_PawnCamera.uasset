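; BP_PawnCamera is a player camera pawn that pans across the map selector.
; On controller change it adds the Enhanced Input mapping, shows the cursor in Game and UI mode, and stores its height.
; The move action pans by speed and delta time, clamping X to map bounds and forcing fixed Y and Z.
; Tick restores the stored height every frame; GetMoney is a stub returning zero.
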(event Input|EnhancedActionEvents|EnhancedInputActionIA_MapSelectorCameraMove
  (params (ActionValue :type Float%20%28double-precision%29) (ElapsedSeconds :type Float%20%28double-precision%29) (TriggeredSeconds :type Float%20%28double-precision%29) (InputAction :type Input%20Action%20Object%20Reference :default "/Game/_Protocol/BP/Input/Actions/IA_MapSelectorCameraMove.IA_MapSelectorCameraMove"))
  (bind _returnvalue (Utilities|Time|GetWorldDeltaSeconds))
  (bind _panspeed (Variables|Default|GetPanSpeed))
  ;[0.15 0.15 0.15 0.5] Camera
  (Transformation|SetActorLocation (Math|Vector|MakeVector (Math|Float|Clamp(Float) (.x (+ (+ (* (Transformation|GetActorRightVector) (* ActionValue _panspeed _returnvalue)) (* (Transformation|GetActorForwardVector) (* ActionValue _panspeed _returnvalue))) (Transformation|GetActorLocation))) (Variables|Default|GetMapMin) (Variables|Default|GetMapMax)) 2.37e+03 22688.0) false false))

(event EventControllerChanged
  (params (OldController :type Controller%20Object%20Reference) (NewController :type Controller%20Object%20Reference))
  (bind _returnvalue (Game|GetPlayerController 0))
  ;[0.15 0.15 0.15 0.5] Beginplay
  (bind _asplayer_controller (Utilities|Casting|CastToPlayerController NewController))
  (Input|AddMappingContext (PlayerController|LocalPlayerSubsystems|GetEnhancedInputLocalPlayerSubsystem _asplayer_controller) "/Game/_Protocol/BP/Input/IMC_Default.IMC_Default" 1 "(bIgnoreAllPressedKeysUntilRelease=True,bForceImmediately=False,bNotifyUserSettings=False)")
  (Variables|/Script/Engine.PlayerController|SetbShowMouseCursor _returnvalue true)
  (Input|SetInputModeGameandUI _returnvalue 0 "DoNotLock" true false)
  (Variables|Default|SetZ (.z (Transformation|GetActorLocation))))

(event EventTick
  (params (DeltaSeconds :type Float%20%28single-precision%29))
  (bind _returnvalue (Transformation|GetActorLocation))
  ;[0.15 0.15 0.15 0.5] Tick
  (Transformation|SetActorLocation (Math|Vector|MakeVector (.x _returnvalue) (.y _returnvalue) (Variables|Default|GetZ)) false false))

(fn ConstructionScript)

(fn GetMoney
  (return 0))