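; BP_GhostSupport is a tower Blueprint, by its name the ghost version of a support tower.
; On BeginPlay it calls FillRange, which gathers eight separate range variables into the Ranges array and returns it.
; Its construction script only runs the parent's, and no other logic is defined here.
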(event EventBeginPlay
  (CallFunction|FillRange))

(fn ConstructionScript
  (|CallParentFunction))

(fn FillRange
  (bind _output_get (Variables|Default|SetRanges (Utilities|Array|MakeArray (Variables|Default|GetRange) (Variables|Default|GetRange2) (Variables|Default|GetRange3) (Variables|Default|GetRange4) (Variables|Default|GetRange5) (Variables|Default|GetRange6) (Variables|Default|GetRange7) (Variables|Default|GetRange8))))
  (return _output_get))